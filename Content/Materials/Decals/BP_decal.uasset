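; BP_decal is a decal Blueprint that shows a randomly chosen material from its DecalArray.
; The construction script picks a random array entry and sets it on the Decal component, so the choice is rerolled whenever construction reruns.
; The EventGraph holds a disconnected copy of the same logic that never runs, and the Random variable is unused.
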(fn `UserConstructionScript`
  (bind _decalarray (`self.DecalArray`))
  (`DecalComponent.SetDecalMaterial` (`self.Decal`) (`|GetArrayItem` _decalarray (`KismetMathLibrary.RandomInteger` (`KismetArrayLibrary.Array_Length` _decalarray)))))