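; BP_rock is a configurable rock prop that sets up its mesh and material in the construction script.
; The RockType enum picks one of five thin or fat rock static meshes for the Rock component.
; It then creates a dynamic instance of RockMat, feeds it the normal intensity, texture tiling and texture blend variables, and applies it to the mesh.
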(fn `UserConstructionScript`
  (bind _rock (`self.Rock`))
  (switch `/Game/StaticMeshes/Rocks/RockType` (`self.RockType`)
    (:`NewEnumerator0`
      (`StaticMeshComponent.SetStaticMesh` _rock "/Game/StaticMeshes/Rocks/SM_Rock_01.SM_Rock_01"))
    (:`NewEnumerator1`
      (`StaticMeshComponent.SetStaticMesh` _rock "/Game/StaticMeshes/Rocks/SM_Rock_02.SM_Rock_02"))
    (:`NewEnumerator2`
      (`StaticMeshComponent.SetStaticMesh` _rock "/Game/StaticMeshes/Rocks/SM_Rock_05.SM_Rock_05"))
    (:`NewEnumerator3`
      (`StaticMeshComponent.SetStaticMesh` _rock "/Game/StaticMeshes/Rocks/SM_Rock_03.SM_Rock_03"))
    (:`NewEnumerator4`
      (`StaticMeshComponent.SetStaticMesh` _rock "/Game/StaticMeshes/Rocks/SM_Rock_04.SM_Rock_04")))
  (bind _returnvalue (`KismetMaterialLibrary.CreateDynamicMaterialInstance` (`self.Rock_Mat`)))
  (`MaterialInstanceDynamic.SetScalarParameterValue` _returnvalue "Normal Intensity" (`self.Intensity`))
  (`MaterialInstanceDynamic.SetScalarParameterValue` _returnvalue "TextureTiling" (`self.Tiling`))
  (`MaterialInstanceDynamic.SetScalarParameterValue` _returnvalue "TextureBlend" (`self.Blend`))
  (`PrimitiveComponent.SetMaterial` (`self.Rock`) 0 _returnvalue))