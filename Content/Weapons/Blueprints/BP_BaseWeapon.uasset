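; Base weapon Blueprint that plays an attack montage on AttackCall and applies fixed damage to actors its collider overlaps.
; CollidedActors limits damage to one hit per actor until the montage's notify end clears the list, with player pawn 0 as damage causer.
; Tick checks WeaponDurability and only prints a break message at zero or below; the DamageValue replication handler is empty.
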(event `self.WeaponCollider.OnComponentBeginOverlap`
  (params (OverlappedComponent :type "PrimitiveComponent Object Reference") (OtherActor :type "Actor Object Reference") (OtherComp :type "PrimitiveComponent Object Reference") (OtherBodyIndex :type Integer) (bFromSweep :type Boolean) (SweepResult :type "HitResult Structure (by ref)"))
  (bind _collidedactors (`self.CollidedActors`))
  ;[1 0.0102 0.03009] Weapon
  (if (not (`KismetArrayLibrary.Array_Contains` _collidedactors OtherActor))
    (`KismetArrayLibrary.Array_AddUnique` _collidedactors OtherActor)
    (`GameplayStatics.ApplyDamage` OtherActor 5.0 null (`GameplayStatics.GetPlayerPawn` 0))))

(event `AnimationEnd`
  ;[1 0.0102 0.03009] Weapon
  (`KismetArrayLibrary.Array_Clear` (`self.CollidedActors`)))

(event `WeaponBrokeCheck`
  ;[1 0.0102 0.03009] Weapon
  (if (<= (`self.WeaponDurability`) 0)
    (`KismetSystemLibrary.PrintString` "WeaponBreak")))

(event `self.ReceiveTick`
  (params (DeltaSeconds :type "Float (single-precision)"))
  ;[1 0.0102 0.03009] Weapon
  (`self.WeaponBrokeCheck`))

(event `AttackCall`
  ;[1 0.0102 0.03009] Player presses attack button
  (`|PlayMontage` null (`self.WeaponAnim`)
    (:`OnNotifyEnd`
      (`self.AnimationEnd`))))

(fn `OnRep_DamageValue`)

(fn `UserConstructionScript`)