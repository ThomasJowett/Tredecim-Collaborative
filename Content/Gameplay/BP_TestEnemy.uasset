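; Test enemy Blueprint with health that takes damage, regenerates over time and prints its value for debugging.
; AnyDamage subtracts from EnemyHP, prints the result and damage causer, and sets IsHit to block healing for a short time.
; Tick calls ReHeal and DisplayHP, whose Delay nodes throttle regeneration and HP printing.
; The heal-block Delay is not restarted by further hits during its countdown.
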(event `self.ReceiveBeginPlay`
  ;[0 0.6869 1] HP
  (set `self.EnemyHP` (`self.EnemyMaxHP`)))

(event `self.ReceiveTick`
  (params (DeltaSeconds :type "Float (single-precision)"))
  ;[0 0.6869 1] HP
  (`self.ReHeal`)
  (`self.DisplayHP`))

(event `self.ReceiveAnyDamage`
  (params (Damage :type "Float (single-precision)") (DamageType :type "DamageType Object Reference") (InstigatedBy :type "Controller Object Reference") (DamageCauser :type "Actor Object Reference"))
  ;[0 0.6869 1] HP
  (bind _output_get (set `self.EnemyHP` (- (`self.EnemyHP`) Damage)))
  (set `self.IsHit` true)
  (`self.BlockHealTimer`)
  (`KismetSystemLibrary.PrintString` (`KismetStringLibrary.Conv_DoubleToString` _output_get))
  (`KismetSystemLibrary.PrintString` (`KismetSystemLibrary.GetDisplayName` DamageCauser)))

(event `BlockHealTimer`
  ;[0 0.6869 1] HP
  (`KismetSystemLibrary.Delay` 2.0)
  (set `self.IsHit` false))

(event `DisplayHP`
  ;[0 0.6869 1] HP
  (`KismetSystemLibrary.Delay` 0.5)
  (`KismetSystemLibrary.PrintString` (`KismetStringLibrary.Conv_DoubleToString` (stale `ReHeal` _output_get))))

(event `ReHeal`
  ;[0 0.6869 1] HP
  (if (`self.IsHit`)
    _
    (elif (< (`self.EnemyHP`) (`self.EnemyMaxHP`))
      (`KismetSystemLibrary.Delay` 0.2)
      (bind _output_get (set `self.EnemyHP` (+ (`self.EnemyHP`) 1.0))))))

(fn `UserConstructionScript`)