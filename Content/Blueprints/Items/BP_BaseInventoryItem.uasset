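; Base Blueprint for inventory items that the player picks up by interacting with them.
; Its interact function adds one of the item's own class to the interacting player's Inventory.
; On success it removes its UI widget, destroys the actor and returns the parent's interact result; on failure it returns false.
; The event graph is unused, and the construction script only calls the parent's.
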(fn `Interact_BI`
  (params (PlayerRef :type "/Game/Blueprints/CH_ThirdPerson Object Reference"))
  (returns (PickedUp :type Boolean))
  (bind _success (`/Game/Blueprints/Components/BP_Inventory.AddItem` (`/Game/Blueprints/CH_ThirdPerson.Inventory` PlayerRef) (`GameplayStatics.GetObjectClass` self) 1))
  (if _success
    (`Widget.RemoveFromParent` (`self.UI Ref`))
    (`self.K2_DestroyActor`)
    (bind _pickedup (`parent.Interact_BI` null))
    (return _pickedup)
    (else
      (return false))))

(fn `UserConstructionScript`
  (`parent.UserConstructionScript`))