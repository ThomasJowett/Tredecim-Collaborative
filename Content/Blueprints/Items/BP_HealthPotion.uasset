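; BP_HealthPotion is a usable item that heals the character who uses it.
; It overrides UseItem to call TakeDamage on the character's Health with a negated HealAmount, so healing reuses the damage path, then returns the parent UseItem result.
; The event graph holds only disabled default events, and the construction script just calls its parent.
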(fn `UseItem`
  (params (CharacterRef :type "/Game/Blueprints/CH_ThirdPerson Object Reference"))
  (returns (`Item Was Used` :type Boolean))
  (`/Game/Blueprints/Components/BP_Health.TakeDamage` (`/Game/Blueprints/CH_ThirdPerson.Health` CharacterRef) (* -1 (`self.HealAmount`)))
  (bind _item_was_used (`parent.UseItem` CharacterRef))
  (return _item_was_used))

(fn `UserConstructionScript`
  (`parent.UserConstructionScript`))