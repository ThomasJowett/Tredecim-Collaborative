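; Base pickup item actor that players can interact with to add it to their inventory.
; Interface calls show or hide a UI_Interact prompt, which is created on first display and reused afterward.
; Interacting adds one of the actor's own class to the character's BPInventory, then on success removes the prompt, destroys the actor and debug-prints the slot contents.
; UseItem is an empty stub.
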(event `/Game/Blueprints/Interfaces/BI_IsInteractable.DisplayMessage_BI`
  (params (PlayerRef :type "/Game/Blueprints/CH_ThirdPerson Object Reference"))
  (bind _ui_ref (`self.UI Ref`))
  ;[1 1 1] When in close vicinity of item, show Interact UI and allow for player input
  (`/Engine/EditorBlueprintResources/StandardMacros.IsValid` _ui_ref
    (:`Is Valid`
      (`Widget.SetVisibility` _ui_ref "Visible"))
    (:`Is Not Valid`
      (bind _asplayer_controller (cast `PlayerController` (`Pawn.GetController` PlayerRef)))
      (bind _returnvalue (`|CreateWidget` "/Game/UI/Widgets/UI_Interact.UI_Interact_C" _asplayer_controller self))
      (bind _output_get (set `self.UI Ref` _returnvalue))
      (`UserWidget.AddToViewport` _output_get 0))))

(event `/Game/Blueprints/Interfaces/BI_IsInteractable.HideMessage_BI`
  ;[1 1 1] Remove UI
  (`Widget.SetVisibility` (`self.UI Ref`) "Hidden"))

(fn `Interact_BI`
  (params (PlayerRef :type "/Game/Blueprints/CH_ThirdPerson Object Reference"))
  (returns (PickedUp :type Boolean))
  (bind _asch_third_person (cast `/Game/Blueprints/CH_ThirdPerson` PlayerRef))
  (bind _bp_inventory (`/Game/Blueprints/CH_ThirdPerson.BP_Inventory` _asch_third_person))
  (bind _success (`/Game/Blueprints/Components/BP_Inventory.AddItem` _bp_inventory (`GameplayStatics.GetObjectClass` self) 1))
  (if _success
    (`Widget.RemoveFromParent` (`self.UI Ref`))
    (`self.K2_DestroyActor`)
    (for _array_element (`/Game/Blueprints/Components/BP_Inventory.Slots` _bp_inventory)
      (`KismetSystemLibrary.PrintString` (`KismetSystemLibrary.GetClassDisplayName` (`.ItemClass_2_701FE76C4B15DAF086A2F4B6B79A8CF2` (break `/Game/Blueprints/Structures/InventoryStruct` _array_element)))))
    (return _success)
    (else
      (return false))))

(fn `UseItem`)

(fn `UserConstructionScript`)