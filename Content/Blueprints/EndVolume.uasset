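; EndVolume is a trigger volume that plays the level-ending sequence when a character controlled by PC_ThirdPerson enters its box.
; On overlap it has the controller switch camera through GrabCam, removes all widgets and closes any BP_FinalDoor flagged as the main door.
; After a delay it fades the screen and audio out, then opens the Ben_Blockout level.
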(event `self.Box.OnComponentBeginOverlap`
  (params (OverlappedComponent :type "PrimitiveComponent Object Reference") (OtherActor :type "Actor Object Reference") (OtherComp :type "PrimitiveComponent Object Reference") (OtherBodyIndex :type Integer) (bFromSweep :type Boolean) (SweepResult :type "HitResult Structure (by ref)"))
  (bind _ascharacter (cast `Character` OtherActor))
  (bind _aspc_third_person (cast `/Game/Blueprints/PC_ThirdPerson` (`Pawn.GetController` _ascharacter)))
  (`/Game/Blueprints/PC_ThirdPerson.GrabCam` _aspc_third_person 2 2.0)
  (`WidgetLayoutLibrary.RemoveAllWidgets`)
  (bind _outactors (`GameplayStatics.GetAllActorsOfClass` "/Game/Blueprints/Boss/BossDoor/BP_FinalDoor.BP_FinalDoor_C"))
  (for _array_element _outactors
    (if (`/Game/Blueprints/Boss/BossDoor/BP_FinalDoor.IsMainDoor` _array_element)
      (`/Game/Blueprints/Boss/BossDoor/BP_FinalDoor.CloseDoor` _array_element)
      (`KismetSystemLibrary.Delay` 5.0)
      (`PlayerCameraManager.StartCameraFade` :`self` (`GameplayStatics.GetPlayerCameraManager` 0) :`FromAlpha` 0.0 :`ToAlpha` 1.0 :`Duration` 3.0 :`bShouldFadeAudio` true :`bHoldWhenFinished` true)
      (`KismetSystemLibrary.Delay` 3.0)
      (`GameplayStatics.OpenLevel` "Ben_Blockout"))))

(fn `UserConstructionScript`)