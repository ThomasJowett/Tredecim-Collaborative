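; Stage 1 boss enemy character that attacks the player, reports health to the HUD and calls stage end on death.
; Swipe and Smash attacks play montages, with Smash also spawning BP_P1RangedAtk at the player; a timer ends each attack.
; Hand sphere overlaps apply damage, tracking actors already hit per swing.
; Damage feeds BPHealth and triggers hit reactions on heavy hits, while game mode stage changes set the AI controller class.
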(event `self.ReceiveBeginPlay`
  (bind _asgm_third_person (cast `/Game/Blueprints/GM_ThirdPerson` (`GameplayStatics.GetGameMode`)))
  (bind _output_get (set `self.GameModeRef` _asgm_third_person))
  (add `/Game/Blueprints/GM_ThirdPerson.OnStageChange` _output_get (delegate `StageChanged`))
  (bind _outactors (`GameplayStatics.GetAllActorsOfClass` "/Game/Blueprints/CH_ThirdPerson.CH_ThirdPerson_C"))
  (set `self.PlayerRef` (`|GetArrayItem` _outactors)))

(event `/Game/Blueprints/Interfaces/BI_Enemy.BeginRotation_Bl`
  (bind _capsulecomponent (`self.CapsuleComponent`))
  ;[1 0 0] Rotate During Attack
  (`SceneComponent.K2_SetWorldRotation` _capsulecomponent (`KismetMathLibrary.RInterpTo_Constant` (`SceneComponent.K2_GetComponentRotation` _capsulecomponent) (`KismetMathLibrary.FindLookAtRotation` (`SceneComponent.K2_GetComponentLocation` _capsulecomponent) (`SceneComponent.K2_GetComponentLocation` (`Character.Mesh` (`self.PlayerRef`)))) (`GameplayStatics.GetWorldDeltaSeconds`) 500.0) false false))

(event `StageChanged`
  (params (Stage :type Integer))
  (switch `int` Stage
    (:`1`
      (set `self.AIControllerClass` (`self.Stage1AI`)))
    (:`2`
      (set `self.AIControllerClass` (`self.Stage2AI`)))
    (:`3`
      (set `self.AIControllerClass` (`self.Stage3AI`)))
    (:`4`
      (set `self.AIControllerClass` (`self.Stage4AI`)))))

(event `/Game/Blueprints/Interfaces/BI_Enemy.Attack_BI`
  (params (AttackType :type "/Game/Gameplay/AI/Enums/E_AttackTypes Enum" :default "NewEnumerator0"))
  ;[0.04035 1 0.03873] Begin Attack
  (if (`self.IsAttacking`)
    _
    (elif (not (`self.IsDead`))
      (set `self.IsAttacking` true)
      (switch `/Game/Gameplay/AI/Enums/E_AttackTypes` AttackType
        (:`NewEnumerator0`
          (`AnimInstance.Montage_Play` (`SkeletalMeshComponent.GetAnimInstance` (`self.Mesh`)) (`self.SwipeAttack`) 1.0 "MontageLength" 0.0 true)
          (`KismetSystemLibrary.PrintString` "doing Melee attack"))
        (:`NewEnumerator1`
          (`AnimInstance.Montage_Play` (`SkeletalMeshComponent.GetAnimInstance` (`self.Mesh`)) (`self.SmashAttack`) 1.0 "MontageLength" 0.0 true)
          (`KismetSystemLibrary.PrintString` "doing Ranged attack")
          (`|SpawnActorFromClass` "/Game/Blueprints/BP_P1RangedAtk.BP_P1RangedAtk_C" (`self.GetTransform` (`self.PlayerRef`)) "Undefined" "OverrideRootScale" null null)))
      (`KismetSystemLibrary.K2_SetTimerDelegate` (delegate `/Game/Blueprints/Interfaces/BI_Enemy.AttackEnd_BI`) 5.0))))

(event `/Game/Blueprints/Interfaces/BI_Enemy.AttackEnd_BI`
  (set `self.IsAttacking` false)
  (`KismetArrayLibrary.Array_Clear` (`self.ActorsHitThisSwing`)))

(event `/Game/Blueprints/Interfaces/BI_Enemy.ApplyDamage_BI`
  ;[1 0 0] Damage
)

(event `self.ReceiveAnyDamage`
  (params (Damage :type "Float (single-precision)") (DamageType :type "DamageType Object Reference") (InstigatedBy :type "Controller Object Reference") (DamageCauser :type "Actor Object Reference"))
  (bind _bp_health (`self.BP_Health`))
  ;[0 1 0] Take Damage
  (if (not (`self.IsDead`))
    (`/Game/Blueprints/Components/BP_Health.TakeDamage` _bp_health Damage)
    ;[1 1 1] Boss Health UI
    (message `/Game/Blueprints/Interfaces/BI_UI.BossHealth_BI` (`PlayerController.GetHUD` (`GameplayStatics.GetPlayerController` 0)) (`/Game/Blueprints/Components/BP_Health.MaxHealth` _bp_health) (`/Game/Blueprints/Components/BP_Health.CurrentHealth` _bp_health))
    (if (and (>= Damage 10.0) (not (`self.IsDead`)))
      (`AnimInstance.Montage_Play` (`SkeletalMeshComponent.GetAnimInstance` (`self.Mesh`)) "/Game/Animations/Montages/Boss_Hit_Reaction_Montage.Boss_Hit_Reaction_Montage" 1.0 "MontageLength" 0.0 true)
      (set `self.IsAttacking` false))))

(event `self.Die_BI`
  (set `self.IsDead` true)
  (`AnimInstance.Montage_Play` (`SkeletalMeshComponent.GetAnimInstance` (`self.Mesh`)) "/Game/Animations/Montages/Boss_dying_Montage.Boss_dying_Montage" 1.0 "MontageLength" 0.0 true)
  (`PrimitiveComponent.SetCollisionEnabled` (`self.CapsuleComponent`) "NoCollision")
  (`KismetSystemLibrary.Delay` 3.0)
  (`self.Stage1End`)
  (`self.K2_DestroyActor`))

(event `self.AttackSphereLeft.OnComponentBeginOverlap`
  (params (OverlappedComponent :type "PrimitiveComponent Object Reference") (OtherActor :type "Actor Object Reference") (OtherComp :type "PrimitiveComponent Object Reference") (OtherBodyIndex :type Integer) (bFromSweep :type Boolean) (SweepResult :type "HitResult Structure (by ref)"))
  (if (== OtherActor self)
    _
    (elif (`self.IsAttacking`)
      (if (not (`KismetArrayLibrary.Array_Contains` (`self.ActorsHitThisSwing`) OtherActor))
        (`GameplayStatics.ApplyDamage` OtherActor (`self.Damage`) null self)
        (`KismetArrayLibrary.Array_AddUnique` (`self.ActorsHitThisSwing`) OtherActor)))))

(event `self.AttackSphereRight.OnComponentBeginOverlap`
  (params (OverlappedComponent :type "PrimitiveComponent Object Reference") (OtherActor :type "Actor Object Reference") (OtherComp :type "PrimitiveComponent Object Reference") (OtherBodyIndex :type Integer) (bFromSweep :type Boolean) (SweepResult :type "HitResult Structure (by ref)"))
  (if (`self.IsAttacking`)
    (if (not (`KismetArrayLibrary.Array_Contains` (`self.ActorsHitThisSwing`) OtherActor))
      (`GameplayStatics.ApplyDamage` null (`self.Damage`))
      (`KismetArrayLibrary.Array_AddUnique` (`self.ActorsHitThisSwing`) OtherActor))))

(fn `IsAlive_BI`
  (returns (IsAlive :type Boolean))
  (return (not (`self.IsDead`))))

(fn `IsTargetable`
  (returns (`Can Be Targeted` :type Boolean))
  (bind _isalive (`self.IsAlive_BI`))
  (return _isalive))

(fn `OnDeselected`
  (returns (`Was Deselected` :type Boolean))
  (return false))

(fn `OnSelected`
  (returns (`Was Selected` :type Boolean))
  (return false))

(fn `UserConstructionScript`)