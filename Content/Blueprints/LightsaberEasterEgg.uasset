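; Easter egg actor that reveals a lightsaber and lets a CH_ThirdPerson character pick it up as a weapon.
; Overlapping the Box plays a timeline animating the saber mesh's location and rotation along with spotlight intensity.
; Overlapping Pickup spawns a Lightsaber actor into the character's WeaponInventory, switches weapons and destroys the display component.
; A second timeline then drives the spotlight intensity.
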(event `Play Animation`
  (bind _spotlight (`self.SpotLight`))
  (bind _lightsaber (`self.Lightsaber`))
  (`LightComponent.SetIntensity` _spotlight 0.0)
  (bind (_direction _intensity _lightsaber_position _lightsaber_rotation) (`Timeline|Timeline_0`)
    (:`Update`
      (`LightComponent.SetIntensity` _spotlight _intensity)
      (`SceneComponent.K2_SetRelativeLocation` _lightsaber _lightsaber_position false false)
      (`SceneComponent.K2_SetWorldRotation` _lightsaber (`KismetMathLibrary.MakeRotator` (.x _lightsaber_rotation) (.y _lightsaber_rotation) (.z _lightsaber_rotation)) false false))))

(event `self.Box.OnComponentBeginOverlap`
  (params (OverlappedComponent :type "PrimitiveComponent Object Reference") (OtherActor :type "Actor Object Reference") (OtherComp :type "PrimitiveComponent Object Reference") (OtherBodyIndex :type Integer) (bFromSweep :type Boolean) (SweepResult :type "HitResult Structure (by ref)"))
  (`self.Play Animation`))

(event `self.Pickup.OnComponentBeginOverlap`
  (params (OverlappedComponent :type "PrimitiveComponent Object Reference") (OtherActor :type "Actor Object Reference") (OtherComp :type "PrimitiveComponent Object Reference") (OtherBodyIndex :type Integer) (bFromSweep :type Boolean) (SweepResult :type "HitResult Structure (by ref)"))
  (bind _asch_third_person (cast `/Game/Blueprints/CH_ThirdPerson` OtherActor))
  (bind _returnvalue (`|SpawnActorFromClass` "/Game/Blueprints/Lightsaber.Lightsaber_C" (`KismetMathLibrary.MakeTransform` (0.0 0.0 0.0)) "Undefined" "OverrideRootScale" null null null))
  (bind _weaponinventory (`/Game/Blueprints/CH_ThirdPerson.WeaponInventory` _asch_third_person))
  (`/Game/Blueprints/Components/BP_WeaponInventory.PickUpWeapon` _weaponinventory _returnvalue)
  (`/Game/Blueprints/Components/BP_WeaponInventory.SwitchWeapons` _weaponinventory)
  (`ActorComponent.K2_DestroyComponent` (`self.Lightsaber`))
  (bind (_direction _newtrack_0) (`Timeline|Timeline_1`)
    (:`Update`
      (`LightComponent.SetIntensity` (`self.SpotLight`) _newtrack_0))))

(fn `UserConstructionScript`)