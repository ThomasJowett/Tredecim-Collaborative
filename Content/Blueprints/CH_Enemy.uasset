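; CH_Enemy is a spider enemy character that melee-attacks nearby actors and can be targeted while alive.
; Interface events play the attack montage, guarded by attacking and death flags, and damage every other actor overlapping AttackSphere.
; That sphere's overlap events also tell the controller when something enters or leaves range.
; Incoming damage goes to BPHealth, and the death event enables ragdoll physics on the mesh.
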(event `/Game/Blueprints/Interfaces/BI_Enemy.Attack_BI`
  ;[0.04035 1 0.03873] Begin Attack
  (if (`self.IsAttacking`)
    _
    (elif (not (`self.IsDead`))
      (set `self.IsAttacking` true)
      (`AnimInstance.Montage_Play` (`SkeletalMeshComponent.GetAnimInstance` (`self.Mesh`)) "/Game/SkeletalMeshes/Spider/Animations/Spider_attack.Spider_attack" 1.0 "MontageLength" 0.0 true))))

(event `/Game/Blueprints/Interfaces/BI_Enemy.AttackEnd_BI`
  (set `self.IsAttacking` false))

(event `/Game/Blueprints/Interfaces/BI_Enemy.ApplyDamage_BI`
  ;[0.04035 1 0.03873] Damage
  (for _array_element (`PrimitiveComponent.GetOverlappingActors` (`self.AttackSphere`) null)
    (if (!= _array_element self)
      (`GameplayStatics.ApplyDamage` _array_element (`self.Damage`)))))

(event `self.AttackSphere.OnComponentBeginOverlap`
  (params (OverlappedComponent :type "PrimitiveComponent Object Reference") (OtherActor :type "Actor Object Reference") (OtherComp :type "PrimitiveComponent Object Reference") (OtherBodyIndex :type Integer) (bFromSweep :type Boolean) (SweepResult :type "HitResult Structure (by ref)"))
  ;[0.04035 1 0.03873] Player In range
  (message `/Game/Blueprints/Interfaces/BI_EnemyController.IsInRange_BI` (`self.GetController`) true))

(event `self.AttackSphere.OnComponentEndOverlap`
  (params (OverlappedComponent :type "PrimitiveComponent Object Reference") (OtherActor :type "Actor Object Reference") (OtherComp :type "PrimitiveComponent Object Reference") (OtherBodyIndex :type Integer))
  ;[0.04035 1 0.03873] Player In range
  (message `/Game/Blueprints/Interfaces/BI_EnemyController.IsInRange_BI` (`self.GetController`) false))

(event `self.ReceiveAnyDamage`
  (params (Damage :type "Float (single-precision)") (DamageType :type "DamageType Object Reference") (InstigatedBy :type "Controller Object Reference") (DamageCauser :type "Actor Object Reference"))
  ;[0 1 0] Take Damage
  (`/Game/Blueprints/Components/BP_Health.TakeDamage` (`self.BP_Health`) Damage))

(event `self.Die_BI`
  (set `self.IsDead` true)
  (`PrimitiveComponent.SetSimulatePhysics` (`self.Mesh`) true))

(fn `IsAlive_BI`
  (returns (IsAlive :type Boolean))
  (return (not (`self.IsDead`))))

(fn `IsTargetable`
  (returns (`Can Be Targeted` :type Boolean))
  (bind _isalive (`self.IsAlive_BI`))
  (return _isalive))

(fn `OnDeselected`
  (returns (`Was Deselected` :type Boolean))
  (return false))

(fn `OnSelected`
  (returns (`Was Selected` :type Boolean))
  (return false))

(fn `UserConstructionScript`)