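; Stage 2 boss enemy character that turns to face the player every tick and performs melee or ranged montage attacks.
; Melee damages each actor once per swing through the left attack sphere; ranged spawns an attack on the ground beneath the player, with a cooldown.
; Damage feeds BPHealth and the boss HUD, sometimes triggering hit reactions.
; GameMode stage changes set AIControllerClass, and the fountain barrier toggles invulnerability.
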(event `self.ReceiveTick`
  (params (DeltaSeconds :type "Float (single-precision)"))
  (bind (_returnvalue_roll _returnvalue_pitch _returnvalue_yaw) (`KismetMathLibrary.BreakRotator` (`KismetMathLibrary.FindLookAtRotation` (`SceneComponent.K2_GetComponentLocation` (`self.Mesh`)) (`self.K2_GetActorLocation` (`GameplayStatics.GetPlayerPawn` 0)))))
  ;[0 0.1243 1] STAGE 2 LOOK TOWARDS PLAYER TEST
  (`self.K2_SetActorRotation` (`KismetMathLibrary.MakeRotator` 0.0 0.0 _returnvalue_yaw)))

(event `/Game/Blueprints/Interfaces/BI_Enemy.BeginDamage_BI`
  ;[1 1 1] Damage
  (set `self.IsAttacking` true))

(event `/Game/Blueprints/Interfaces/BI_Enemy.EndDamage_BI`
  ;[1 1 1] Damage
  (set `self.IsAttacking` false)
  (`KismetArrayLibrary.Array_Clear` (`self.ActorsHitThisSwing`)))

(event `self.AttackSphereLeft.OnComponentBeginOverlap`
  (params (OverlappedComponent :type "PrimitiveComponent Object Reference") (OtherActor :type "Actor Object Reference") (OtherComp :type "PrimitiveComponent Object Reference") (OtherBodyIndex :type Integer) (bFromSweep :type Boolean) (SweepResult :type "HitResult Structure (by ref)"))
  ;[1 1 1] Applying Damage to overlapped actors
  (if (== OtherActor self)
    _
    (elif (`self.IsAttacking`)
      (if (not (`KismetArrayLibrary.Array_Contains` (`self.ActorsHitThisSwing`) OtherActor))
        (`GameplayStatics.ApplyDamage` OtherActor (`self.Damage`) null self)
        (`KismetArrayLibrary.Array_AddUnique` (`self.ActorsHitThisSwing`) OtherActor)))))

(event `self.ReceiveBeginPlay`
  ;[1 1 1] Event Begin Play
  (`/Game/Blueprints/Components/BP_IKfoot.Initialize` (`self.BP_IKfoot`) (`self.CapsuleComponent`) (`self.Mesh`))
  (bind _asgm_third_person (cast `/Game/Blueprints/GM_ThirdPerson` (`GameplayStatics.GetGameMode`)))
  (bind _output_get (set `self.GameModeRef` _asgm_third_person))
  (add `/Game/Blueprints/GM_ThirdPerson.OnStageChange` _output_get (delegate `StageChanged`))
  (bind _outactors (`GameplayStatics.GetAllActorsOfClass` "/Game/Blueprints/CH_ThirdPerson.CH_ThirdPerson_C"))
  (set `self.PlayerRef` (`|GetArrayItem` _outactors))
  ;[1 1 1] Set Boss Invunerable
  (bind _outactors_2 (`GameplayStatics.GetAllActorsOfClass` "/Game/Blueprints/Boss/FountainBarrier/BossFountainBarrier.BossFountainBarrier_C"))
  (add `/Game/Blueprints/Boss/FountainBarrier/BossFountainBarrier.BarrierToggle` (`|GetArrayItem` _outactors_2) (delegate `SetBossInvunerable`))
  ;[1 1 1] Health Refill
  (message `/Game/Blueprints/Interfaces/BI_UI.RefillBossHealth_BI` (`PlayerController.GetHUD` (`GameplayStatics.GetPlayerController` 0))))

(event `StageChanged`
  (params (Stage :type Integer))
  ;[1 1 1] Event Begin Play
  (switch `int` Stage
    (:`1`
      (set `self.AIControllerClass` (`self.Stage1AI`)))
    (:`2`
      (set `self.AIControllerClass` (`self.Stage2AI`)))
    (:`3`
      (set `self.AIControllerClass` (`self.Stage3AI`)))
    (:`4`
      (set `self.AIControllerClass` (`self.Stage4AI`)))))

(event `SetBossInvunerable`
  (params (BarrierOn :type Boolean))
  ;[1 1 1] Set Boss Invunerable
  (if BarrierOn
    (set `self.bCanBeDamaged` false)
    (else
      (set `self.bCanBeDamaged` true))))

(event `self.AttackSphereRight.OnComponentBeginOverlap`
  (params (OverlappedComponent :type "PrimitiveComponent Object Reference") (OtherActor :type "Actor Object Reference") (OtherComp :type "PrimitiveComponent Object Reference") (OtherBodyIndex :type Integer) (bFromSweep :type Boolean) (SweepResult :type "HitResult Structure (by ref)"))
  ;[1 1 1] Applying Damage to overlapped actors
)

(event `/Game/Blueprints/Interfaces/BI_Enemy.Attack_BI`
  (params (AttackType :type "/Game/Blueprints/AI/Enums/E_AttackTypes Enum" :default "NewEnumerator0"))
  (bind _playerref (`self.PlayerRef`))
  (bind (_returnvalue_x _returnvalue_y _returnvalue_z) (`KismetMathLibrary.BreakVector` (`self.K2_GetActorLocation` _playerref)))
  ;[1 1 1] Begin Attack
  (if (and (not (`self.IsDead`)) (not (`self.IsAttacking`)))
    (switch `/Game/Blueprints/AI/Enums/E_AttackTypes` AttackType
      (:`NewEnumerator0`
        ;[1 1 1] Melee Attack
        (`AnimInstance.Montage_Play` (`SkeletalMeshComponent.GetAnimInstance` (`self.Mesh`)) (`self.MeleeAttack`) 1.0 "MontageLength" 0.0 true)
        (`KismetSystemLibrary.PrintString` "doing Melee attack"))
      (:`NewEnumerator1`
        ;[1 1 1] Ranged attack
        (if (not (`self.RangedAttackCooldown`))
          (`AnimInstance.Montage_Play` (`SkeletalMeshComponent.GetAnimInstance` (`self.Mesh`)) (`self.RangedAttack`) 1.0 "MontageLength" 0.0 true)
          (`KismetSystemLibrary.PrintString` "doing Ranged attack")
          (bind _outhit (`KismetSystemLibrary.LineTraceSingle` (`self.K2_GetActorLocation` _playerref) (`KismetMathLibrary.MakeVector` _returnvalue_x _returnvalue_y (+ _returnvalue_z -1000.0)) "TraceTypeQuery1" false (`|MakeArray` _playerref :!type "Actor Object Reference") "Persistent"))
          (`|SpawnActorFromClass` "/Game/Blueprints/Boss/RangedAttackPhase1/BP_P1RangedAtk.BP_P1RangedAtk_C" (`KismetMathLibrary.Conv_VectorToTransform` (`.ImpactPoint` (`GameplayStatics.BreakHitResult` _outhit))) "Undefined" "OverrideRootScale" self self)
          (set `self.RangedAttackCooldown` true)
          (`KismetSystemLibrary.Delay` 2.0)
          (set `self.RangedAttackCooldown` false))))))

(event `self.ReceiveAnyDamage`
  (params (Damage :type "Float (single-precision)") (DamageType :type "DamageType Object Reference") (InstigatedBy :type "Controller Object Reference") (DamageCauser :type "Actor Object Reference"))
  (bind _bp_health (`self.BP_Health`))
  ;[1 1 1] Receive Damage
  ;;[1 1 1] Take Damage
  (if (not (or (== InstigatedBy self) (`self.IsDead`)))
    (`/Game/Blueprints/Components/BP_Health.TakeDamage` _bp_health Damage)
    ;;[1 1 1] Boss Health UI
    (message `/Game/Blueprints/Interfaces/BI_UI.BossHealth_BI` (`PlayerController.GetHUD` (`GameplayStatics.GetPlayerController` 0)) (`/Game/Blueprints/Components/BP_Health.MaxHealth` _bp_health) (`/Game/Blueprints/Components/BP_Health.CurrentHealth` _bp_health))
    (if (and (>= Damage 10.0) (not (`self.IsDead`)))
      (if (`KismetMathLibrary.RandomBool`)
        (`AnimInstance.Montage_Play` (`SkeletalMeshComponent.GetAnimInstance` (`self.Mesh`)) "/Game/Animations/Montages/Boss_Hit_Reaction_Montage.Boss_Hit_Reaction_Montage" 1.0 "MontageLength" 0.0 true)
        (set `self.IsAttacking` false)))))

(event `/Game/Blueprints/Interfaces/BI_Death.Die_BI`
  ;[1 1 1] Receive Damage
  ;;[1 1 1] OnDeath
  (set `self.IsDead` true)
  (`AnimInstance.Montage_Play` (`SkeletalMeshComponent.GetAnimInstance` (`self.Mesh`)) "/Game/Animations/Montages/Boss_dying_Montage.Boss_dying_Montage" 1.0 "MontageLength" 0.0 true)
  (`PrimitiveComponent.SetCollisionEnabled` (`self.CapsuleComponent`) "NoCollision")
  (`KismetSystemLibrary.Delay` 3.0)
  (`self.K2_DestroyActor`))

(fn `IsAlive_BI`
  (returns (IsAlive :type Boolean))
  (return (not (`self.IsDead`))))

(fn `IsTargetable`
  (returns (`Can Be Targeted` :type Boolean))
  (bind _isalive (`/Game/Blueprints/Interfaces/BI_Death.IsAlive_BI`))
  (return _isalive))

(fn `OnDeselected`
  (returns (`Was Deselected` :type Boolean))
  (return false))

(fn `OnSelected`
  (returns (`Was Selected` :type Boolean))
  (return false))

(fn `UserConstructionScript`)