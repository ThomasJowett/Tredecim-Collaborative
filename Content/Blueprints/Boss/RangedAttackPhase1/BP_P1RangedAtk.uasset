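; Hazard actor for the boss's phase 1 ranged attack that damages and launches whatever player character overlaps it.
; After a short delay, a timeline nudges its cube upward, and the actor destroys itself a few seconds later.
; Overlap applies ranged-type damage, then launches CH_ThirdPerson upward with random horizontal force.
; A delayed loop sends ragdoll interface messages until vertical velocity is zero, then re-enables walking.
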(event `self.ReceiveBeginPlay`
  (bind _cube (`self.Cube`))
  (bind _returnvalue (`SceneComponent.K2_GetComponentLocation` _cube))
  ;[0 1 0.05863] Rnaged Attack
  (`KismetSystemLibrary.Delay` 1.2)
  (bind (_direction _alpha) (`Timeline|Timeline_0`)
    (:`Update`
      (`SceneComponent.K2_SetWorldLocation` _cube (`KismetMathLibrary.VLerp` _returnvalue (`KismetMathLibrary.MakeVector` (.x _returnvalue) (.y _returnvalue) (+ (.z _returnvalue) 7.0)) _alpha) false false))
    (:`Finished`
      _))
  (`KismetSystemLibrary.Delay` 4.0)
  (`self.K2_DestroyActor`))

(event `self.ReceiveActorBeginOverlap`
  (params (OtherActor :type "Actor Object Reference"))
  (bind _returnvalue (`KismetMathLibrary.RandomFloatInRange` (`self.LaunchValueMin`) (`self.LaunchValueMax`)))
  ;[0 1 0.05863] Rnaged Attack
  (`GameplayStatics.ApplyDamage` OtherActor 5.0 null self "/Game/Blueprints/DamageTypes/BP_RangedDT.BP_RangedDT_C")
  (bind _asch_third_person (cast `/Game/Blueprints/CH_ThirdPerson` OtherActor))
  (`Character.LaunchCharacter` _asch_third_person (`KismetMathLibrary.MakeVector` _returnvalue _returnvalue 1000.0) false false)
  (`KismetSystemLibrary.Delay` 0.2 :!label _label)
  (message `/Game/Blueprints/Interfaces/BI_Character.Ragdoll_BI` _asch_third_person)
  (`KismetSystemLibrary.Delay` 2.5)
  (bind (_returnvalue_x _returnvalue_y _returnvalue_z) (`KismetMathLibrary.BreakVector` (`self.GetVelocity` _asch_third_person)))
  (if (== _returnvalue_z 0.0)
    (message `/Game/Blueprints/Interfaces/BI_Character.Ragdoll_BI` _asch_third_person)
    (message `/Game/Blueprints/Interfaces/BI_Character.EnableWalking_BI` _asch_third_person)
    (else
      (goto _label))))

(fn `UserConstructionScript`)