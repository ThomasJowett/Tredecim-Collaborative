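; BP_BuffRangedAttack is a ranged slash projectile, apparently the buffed variant of the player's ranged attack.
; On BeginPlay, a timeline moves the Cube along its forward vector each update, with a frame-rate-scaled step weighted by the timeline's alpha, then destroys the actor when finished.
; SlashCollider applies fixed damage to any overlapping actor using the BP_PlayerRangedDT damage type, without destroying the projectile.
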(event `self.ReceiveBeginPlay`
  (bind _cube (`self.Cube`))
  (bind _returnvalue (`SceneComponent.K2_GetComponentToWorld` _cube))
  ;[0.02247 1 0] Ranged Attack Movement
  (bind (_direction _alpha) (`Timeline|Lerp`)
    (:`Update`
      (`SceneComponent.K2_SetWorldTransform` _cube (`KismetMathLibrary.TLerp` _returnvalue (`KismetMathLibrary.MakeTransform` (+ (* (`KismetMathLibrary.Normal` (`SceneComponent.GetForwardVector` _cube)) (* (`GameplayStatics.GetWorldDeltaSeconds`) 750.0)) (.location _returnvalue)) (.rotation _returnvalue) (.scale _returnvalue)) _alpha) false false))
    (:`Finished`
      (`self.K2_DestroyActor`))))

(event `self.SlashCollider.OnComponentBeginOverlap`
  (params (OverlappedComponent :type "PrimitiveComponent Object Reference") (OtherActor :type "Actor Object Reference") (OtherComp :type "PrimitiveComponent Object Reference") (OtherBodyIndex :type Integer) (bFromSweep :type Boolean) (SweepResult :type "HitResult Structure (by ref)"))
  (`GameplayStatics.ApplyDamage` OtherActor 5.0 null self "/Game/Blueprints/DamageTypes/BP_PlayerRangedDT.BP_PlayerRangedDT_C"))

(fn `UserConstructionScript`)