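; BP_TestDoor is a test door actor that shows an interaction prompt but has no opening logic.
; Its display event lazily creates a UI_Interact widget for the player's controller, passing itself and a vertical offset, then reuses it by toggling visibility with the hide event.
; GetInfoBI supplies the "Open Door" name and "Use" text, while InteractBI is a stub returning false.
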(event `/Game/Blueprints/Interfaces/BI_IsInteractable.DisplayMessage_BI`
  (params (PlayerRef :type "/Game/Blueprints/CH_ThirdPerson Object Reference"))
  (bind _ui_ref (`self.UI Ref`))
  (`/Engine/EditorBlueprintResources/StandardMacros.IsValid` _ui_ref
    (:`Is Valid`
      (`Widget.SetVisibility` _ui_ref "Visible"))
    (:`Is Not Valid`
      (bind _asplayer_controller (cast `PlayerController` (`Pawn.GetController` PlayerRef)))
      (bind _returnvalue (`|CreateWidget` "/Game/UI/Widgets/UI_Interact.UI_Interact_C" _asplayer_controller self (0.0 0.0 -350.0)))
      (bind _output_get (set `self.UI Ref` _returnvalue))
      (`UserWidget.AddToViewport` _output_get 0))))

(event `/Game/Blueprints/Interfaces/BI_IsInteractable.HideMessage_BI`
  (`Widget.SetVisibility` (`self.UI Ref`) "Hidden"))

(fn `GetInfo_BI`
  (returns (ItemInfo :type "/Game/Blueprints/Structures/ItemInfoStruct Structure"))
  (return (make `/Game/Blueprints/Structures/ItemInfoStruct` "Open Door" "" "Use")))

(fn `Interact_BI`
  (params (PlayerRef :type "/Game/Blueprints/CH_ThirdPerson Object Reference"))
  (returns (PickedUp :type Boolean))
  (return false))

(fn `UserConstructionScript`)