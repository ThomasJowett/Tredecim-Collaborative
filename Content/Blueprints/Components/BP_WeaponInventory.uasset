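; Character weapon inventory component that manages main-hand, left-hand and back slots by attaching weapon actors to mesh sockets.
; PickUpWeapon fills free slots or drops the held item to make room.
; SwitchWeapons swaps hand and back weapons, stows or restores shields around two-handers and notifies the AnimInstance.
; An older StoredWeapons array system remains in EventGraph, but SetWeapon is empty, so the sword spawned at BeginPlay is never equipped.
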(event `self.ReceiveBeginPlay`
  (bind _returnvalue (`|SpawnActorFromClass` "/Game/Weapons/WP_Sword.WP_Sword_C" (`KismetMathLibrary.MakeTransform` (0.0 0.0 0.0)) "Undefined" "OverrideRootScale" null null))
  (`self.SetWeapon` _returnvalue))

(event `SetWeapon`
  (params (NewWeapon :type "WP_BaseWeapon Object Reference"))
  ;[0 1 0.03457] Set weapon when called/Two weapon inventory
)

(event `DetachCurrentWeapon`
  ;[0 1 0.03457] Detach Current Weapon
  (`/Engine/EditorBlueprintResources/StandardMacros.IsValid` null
    (:`Is Valid`
      (`SceneComponent.K2_DetachFromComponent` (`Actor.RootComponent` (`|GetArrayItem` (`self.StoredWeapons`) (`self.CurrentWeapon`))) "KeepWorld" "KeepRelative" "KeepRelative" true))))

(event `WeaponSwitch`
  ;[0 1 0.03457] WeaponSwitch
  (bind _result (`/Engine/EditorBlueprintResources/StandardMacros.IncrementInt` (`self.CurrentWeapon`))
    (:`  `
      (if (`KismetArrayLibrary.Array_IsValidIndex` (`self.StoredWeapons`) _result)
        (`self.EquipWeapon` _result)
        (else
          (`self.EquipWeapon` 0)
          (set `self.CurrentWeapon` 0))))))

(event `EquipWeapon`
  (params (WeapToEquip :type Integer))
  (bind _ascharacter (cast `Character` (`self.GetOwner`) :!pure true))
  (bind _output (`|GetArrayItem` (`self.StoredWeapons`) WeapToEquip))
  ;[0 1 0.03457] EquipWeapon
  (`self.DetachCurrentWeapon`)
  (`SceneComponent.K2_DetachFromComponent` (`Actor.RootComponent` _output) "KeepRelative" "KeepRelative" "KeepRelative" true)
  (`Actor.K2_AttachToComponent` (`|GetArrayItem` (`self.StoredWeapons`) (- (`self.CurrentWeapon`) 1)) (`Character.Mesh` _ascharacter) "spine_03Socket" "SnapToTarget" "SnapToTarget" "SnapToTarget" true)
  (`Actor.K2_AttachToComponent` _output (`Character.Mesh` _ascharacter) "hand_rSocket" "SnapToTarget" "SnapToTarget" "SnapToTarget" true))

(fn `AttachToBack`
  (params (Weapon :type "WP_BaseWeapon Object Reference"))
  (bind _rootcomponent (`Actor.RootComponent` Weapon))
  (bind _mesh (`Character.Mesh` (`self.ParentCharacter`)))
  (if (`WP_BaseWeapon.bIsMainHand` Weapon)
    (`SceneComponent.K2_AttachToComponent` _rootcomponent _mesh "BackWeapon" "SnapToTarget" "SnapToTarget" "KeepRelative" true)
    (set `self.BackWeapon` Weapon)
    (elif (`WP_BaseWeapon.bIsTwoHanded` (`self.EquippedWeapon`))
      (`SceneComponent.K2_AttachToComponent` _rootcomponent _mesh "BackShield" "SnapToTarget" "SnapToTarget" "KeepRelative" true)
      (set `self.BackShield` Weapon))))

(fn `AttachToLeftHand`
  (params (Weapon :type "WP_BaseWeapon Object Reference"))
  (`SceneComponent.K2_AttachToComponent` (`Actor.RootComponent` Weapon) (`Character.Mesh` (`self.ParentCharacter`)) "lowerarm_lSocket" "SnapToTarget" "SnapToTarget" "KeepRelative" true)
  (set `self.LeftHandWeapon` Weapon))

(fn `AttachToRightHand`
  (params (Weapon :type "WP_BaseWeapon Object Reference"))
  (`SceneComponent.K2_AttachToComponent` (`Actor.RootComponent` Weapon) (`Character.Mesh` (`self.ParentCharacter`)) "hand_rSocket" "SnapToTarget" "SnapToTarget" "KeepRelative" true)
  (set `self.EquippedWeapon` Weapon))

(fn `DropWeapon`
  (params (Weapon :type "WP_BaseWeapon Object Reference"))
  (`Actor.K2_DetachFromActor` Weapon "KeepWorld" "KeepWorld" "KeepWorld"))

(fn `GetEquippedWeapon`
  (returns (EquippedWeapon :type "WP_BaseWeapon Object Reference"))
  (return (`self.EquippedWeapon`)))

(fn `PickUpWeapon`
  (params (Weapon :type "WP_BaseWeapon Object Reference"))
  (bind _lefthandweapon (`self.LeftHandWeapon`))
  (`/Engine/EditorBlueprintResources/StandardMacros.IsValid` (`self.ParentCharacter`)
    (:`Is Valid`
      (set `WP_BaseWeapon.WeaponOwner` (stale _output_get) Weapon :!label _label)
      (if (`WP_BaseWeapon.bIsMainHand` Weapon)
        (if (== (`self.EquippedWeapon`) null)
          (`self.AttachToRightHand` Weapon)
          (elif (== (`self.BackWeapon`) null)
            (`self.AttachToBack` Weapon)
            (else
              (`self.DropWeapon` (`self.EquippedWeapon`))
              (`self.AttachToRightHand` Weapon))))
        (elif (== _lefthandweapon null)
          (`self.AttachToLeftHand` Weapon :!label _label_2)
          (elif (== (`self.BackShield`) null)
            (`self.AttachToBack` Weapon)
            (else
              (`self.DropWeapon` _lefthandweapon)
              (goto _label_2))))))
    (:`Is Not Valid`
      (bind _ascharacter (cast `Character` (`self.GetOwner`))
        (:`then`
          (bind _output_get (set `self.ParentCharacter` _ascharacter))
          (goto _label))
        (:`CastFailed`
          (`KismetSystemLibrary.PrintString` "Inventory Not attached to actor"))))))

(fn `SwitchWeapons`
  (locals (TempWeaponRef :type "WP_BaseWeapon Object Reference") (TempWeaponRef2 :type "WP_BaseWeapon Object Reference"))
  (bind _backshield (`self.BackShield`))
  (bind _lefthandweapon (`self.LeftHandWeapon`))
  (bind _tempweaponref2 (`local.TempWeaponRef2`))
  (bind _returnvalue (`SkeletalMeshComponent.GetAnimInstance` (`Character.Mesh` (`self.ParentCharacter`))))
  (if (== (`self.BackWeapon`) null)
    _
    (elif (`WP_BaseWeapon.bIsTwoHanded` (`self.BackWeapon`))
      (if (not (== _lefthandweapon null))
        (set `local.TempWeaponRef2` _lefthandweapon)
        (set `self.LeftHandWeapon` null))
      (bind _output_get (set `local.TempWeaponRef` (`self.EquippedWeapon`) :!label _label))
      (`self.AttachToRightHand` (`self.BackWeapon`))
      (`self.AttachToBack` _output_get)
      (`/Engine/EditorBlueprintResources/StandardMacros.IsValid` _tempweaponref2
        (:`Is Valid`
          (`self.AttachToBack` _tempweaponref2))
        (:`Is Not Valid`
          _))
      (if (`WP_BaseWeapon.bIsTwoHanded` (`self.EquippedWeapon`))
        (message `/Game/Blueprints/Interfaces/BI_Animation.SetWeaponType_BI` _returnvalue "NewEnumerator1")
        (else
          (message `/Game/Blueprints/Interfaces/BI_Animation.SetWeaponType_BI` _returnvalue "NewEnumerator0")))
      (elif (`WP_BaseWeapon.bIsTwoHanded` (`self.EquippedWeapon`))
        (if (not (== _backshield null))
          (`self.AttachToLeftHand` _backshield)
          (set `self.BackShield` null)
          (goto _label))
        (else
          (goto _label))))))