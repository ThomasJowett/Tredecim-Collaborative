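; Input buffer Blueprint that stores the most recent key passed to it and exposes a window that can be opened and closed.
; UpdateKey overwrites the stored key whether or not the window is open; its open-state check leads to no action.
; Opening and closing set the state and fire event dispatchers.
; Consuming broadcasts the stored key, then resets it to a fixed enum value, independent of the window state.
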(fn `CloseInputBuffer`
  (set `self.IsOpen` false)
  (`self.OnInputBufferClose`))

(fn `ComsumeInputBuffer`
  (`self.OnInputBufferConsumed` (`self.StoredKey`))
  (set `self.StoredKey` "NewEnumerator2"))

(fn `OpenInputBuffer`
  (set `self.IsOpen` true)
  (`self.OnInputBufferOpen`))

(fn `UpdateKey`
  (params (Key :type "/Game/Blueprints/Enums/E_Input_Buffer_key Enum" :default "NewEnumerator2"))
  (set `self.StoredKey` Key)
  (if (`self.IsOpen`)
    _))