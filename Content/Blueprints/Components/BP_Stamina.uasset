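; Stamina component that gates actions by their stamina cost and regenerates stamina after a delay.
; PerformAction refuses any cost that would leave stamina at zero or below; otherwise it deducts it, pauses regen and restarts the ResetRegen delay timer.
; ResetRegen starts a fast looping timer on RegenStamina, which adds stamina at StamRegenRate until MaxStam is reached.
; BeginPlay starts stamina at maximum.
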(event `ResetRegen`
  (set `self.CanRegen` true)
  (`KismetSystemLibrary.K2_SetTimerDelegate` (delegate `RegenStamina`) 0.02 true))

(event `RegenStamina`
  ;[1 1 1] Stamina Regen
  (if (`self.CanRegen`)
    (if (< (`self.CurrentStam`) (`self.MaxStam`))
      (set `self.CurrentStam` (+ (`self.CurrentStam`) (* 0.02 (`self.StamRegenRate`))))
      (else
        (set `self.CanRegen` false)
        (`KismetSystemLibrary.K2_ClearTimer` null "RegenStamina")))))

(event `self.ReceiveBeginPlay`
  ;[1 1 1] Set Stam to max on play
  (bind _output_get (set `self.CurrentStam` (`self.MaxStam`)))
  (set `self.MaxStam` _output_get))

(fn `PerformAction`
  (params (StaminaCost :type "Float (double-precision)"))
  (returns (CanPerformAction :type Boolean))
  (bind _returnvalue (- (`self.CurrentStam`) StaminaCost))
  (if (<= _returnvalue 0.0)
    (return false) ; If they do not have enough Stamina then they cannot perfom the action
    (else
      (set `self.CurrentStam` _returnvalue)
      (`KismetSystemLibrary.K2_SetTimer` self "ResetRegen" (`self.RegenDelay`))
      (set `self.CanRegen` false)
      (return true))))