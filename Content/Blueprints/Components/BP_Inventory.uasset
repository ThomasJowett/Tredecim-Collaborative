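; Inventory component for the CH_ThirdPerson player, holding a fixed-size array of item class and quantity slots.
; AddItem recursively spreads amounts over slots within the stack limit and returns any remainder, though SearchFreeStack never reports success, so existing stacks are not topped up.
; Cycle functions skip empty slots to select the current item.
; UseItem spawns that item, calls its UseItem on the player and, on success, destroys it and decrements the slot.
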(event `self.ReceiveBeginPlay`
  (`KismetArrayLibrary.Array_Resize` (`self.Slots`) (`self.AmountOfSlots`))
  (bind _asch_third_person (cast `/Game/Blueprints/CH_ThirdPerson` (`self.GetOwner`)))
  (set `self.PlayerRef` _asch_third_person))

(fn `AddItem`
  (params (ItemClass :type "/Game/Blueprints/Items/BP_BasePickUp Class Reference") (Amount :type Integer))
  (returns (Success :type Boolean) (Rest :type Integer))
  (locals (LocalClass :type "/Game/Blueprints/Items/BP_BasePickUp Class Reference") (LocalAmount :type Integer) (FoundIndex :type Integer))
  (bind _returnvalue (+ (`.Quantity_5_9283D68A437DE9AB4BCDCF85F13B1C81` (break `/Game/Blueprints/Structures/InventoryStruct` (`|GetArrayItem` (`self.Slots`) (`local.FoundIndex`)))) (`local.LocalAmount`)))
  (set `local.LocalClass` ItemClass)
  (set `local.LocalAmount` Amount)
  (if (`.CanBeStacked_39_4783A2174BFCEAEC71245E99DB1BDB2B` (break `/Game/Blueprints/Structures/ItemInfoStruct` (defaults `/Game/Blueprints/Components/BP_Inventory` ItemClass)))
    (bind (_succuss _index) (`self.SearchFreeStack` (`local.LocalClass`)))
    (if _succuss
      (set `local.FoundIndex` _index)
      (if (> _returnvalue (`self.MaxStackSize`))
        (set `local.LocalAmount` (- _returnvalue (`self.MaxStackSize`)))
        (`KismetArrayLibrary.Array_Set` (`self.Slots`) (`local.FoundIndex`) (make `/Game/Blueprints/Structures/InventoryStruct` (`local.LocalClass`) (`self.MaxStackSize`)))
        (bind (_success _rest) (`self.AddItem` (`local.LocalClass`) (`local.LocalAmount`)))
        (return true _rest)
        (else
          (`KismetArrayLibrary.Array_Set` (`self.Slots`) (`local.FoundIndex`) (make `/Game/Blueprints/Structures/InventoryStruct` (`local.LocalClass`) _returnvalue))
          (return true 0)))
      (else
        (bind (_success_2 _index_2) (`self.SearchEmptySlot`))
        (if _success_2
          (bind _output_get (set `local.FoundIndex` _index_2))
          (if (> (`local.LocalAmount`) (`self.MaxStackSize`))
            (`KismetArrayLibrary.Array_Set` (`self.Slots`) _output_get (make `/Game/Blueprints/Structures/InventoryStruct` (`local.LocalClass`) (`self.MaxStackSize`)))
            (bind (_success_3 _rest_2) (`self.AddItem` (`local.LocalClass`) (- (`local.LocalAmount`) (`self.MaxStackSize`))))
            (return true _rest_2)
            (else
              (`KismetArrayLibrary.Array_Set` (`self.Slots`) (`local.FoundIndex`) (make `/Game/Blueprints/Structures/InventoryStruct` (`local.LocalClass`) (`local.LocalAmount`)))
              (return true 0)))
          (else
            (return false (`local.LocalAmount`))))))
    (else
      (bind (_success_4 _index_3) (`self.SearchEmptySlot`))
      (if _success_4
        (bind _output_get_2 (set `local.FoundIndex` _index_3))
        (`KismetArrayLibrary.Array_Set` (`self.Slots`) _output_get_2 (make `/Game/Blueprints/Structures/InventoryStruct` (`local.LocalClass`) 1))
        (if (> (`local.LocalAmount`) 1)
          (bind (_success_5 _rest_3) (`self.AddItem` (`local.LocalClass`) (- (`local.LocalAmount`) 1)))
          (return true _rest_3)
          (else
            (return true 0)))
        (else
          (return false (`local.LocalAmount`)))))))

(fn `CycleItemNext`
  (if (not (`self.IsInventoryEmpty`))
    (bind _result (`/Engine/EditorBlueprintResources/StandardMacros.IncrementInt` (`self.CurrentItemIndex`))
      (:`  `
        (if (> (`self.CurrentItemIndex`) (- (`self.AmountOfSlots`) 1))
          (set `self.CurrentItemIndex` 0)
          (else
            (bind _output_get (set `self.CurrentItemIndex` _result))))
        (if (== (`.Quantity_5_9283D68A437DE9AB4BCDCF85F13B1C81` (break `/Game/Blueprints/Structures/InventoryStruct` (`|GetArrayItem` (`self.Slots`) _output_get))) 0)
          (`self.CycleItemNext`))))))

(fn `CycleItemPrevious`
  (if (not (`self.IsInventoryEmpty`))
    (bind _result (`/Engine/EditorBlueprintResources/StandardMacros.DecrementInt` (`self.CurrentItemIndex`))
      (:`  `
        (if (< (`self.CurrentItemIndex`) 0)
          (set `self.CurrentItemIndex` (- (`self.AmountOfSlots`) 1))
          (else
            (set `self.CurrentItemIndex` _result)))
        (if (== (`.Quantity_5_9283D68A437DE9AB4BCDCF85F13B1C81` (break `/Game/Blueprints/Structures/InventoryStruct` (`|GetArrayItem` (`self.Slots`) (`self.CurrentItemIndex`)))) 0)
          (`self.CycleItemPrevious`))))))

(fn `DisplayCurrentIndex`
  (bind _output_itemclass (break `/Game/Blueprints/Structures/InventoryStruct` (`|GetArrayItem` (`self.Slots`) (`self.CurrentItemIndex`))))
  (`KismetSystemLibrary.PrintString` (`KismetSystemLibrary.GetClassDisplayName` _output_itemclass) true true (struct :`G` 1.0 :`B` 0.014685 :`A` 1.0)))

(fn `GetAmountAtIndex`
  (params (Index :type Integer))
  (returns (Quantity :type Integer))
  (return (`.Quantity_5_9283D68A437DE9AB4BCDCF85F13B1C81` (break `/Game/Blueprints/Structures/InventoryStruct` (`|GetArrayItem` (`self.Slots`) Index)))))

(fn `GetItemInfoAtIndex`
  (params (Index :type Integer))
  (returns (EmptySlot :type Boolean) (ItemInfo :type "/Game/Blueprints/Structures/ItemInfoStruct Structure") (Quantity :type Integer))
  (bind (_itemclass _quantity) (break `/Game/Blueprints/Structures/InventoryStruct` (`|GetArrayItem` (`self.Slots`))))
  (if (`KismetSystemLibrary.IsValidClass` _itemclass)
    (return false (defaults `/Game/Blueprints/Components/BP_Inventory` _itemclass) _quantity)
    (else
      (return true (struct) 0))))

(fn `IsInventoryEmpty`
  (returns (IsEmpty :type Boolean))
  (for _array_element (`self.Slots`)
    (if (> (`.Quantity_5_9283D68A437DE9AB4BCDCF85F13B1C81` (break `/Game/Blueprints/Structures/InventoryStruct` _array_element)) 0)
      (return false)))
  (return true))

(fn `IsSlotEmpty`
  (params (Index :type Integer))
  (returns (IsEmpty :type Boolean))
  (return (not (`KismetSystemLibrary.IsValidClass` (`.ItemClass_2_701FE76C4B15DAF086A2F4B6B79A8CF2` (break `/Game/Blueprints/Structures/InventoryStruct` (`|GetArrayItem` (`self.Slots`) Index)))))))

(fn `SearchEmptySlot`
  (returns (Success :type Boolean) (Index :type Integer))
  (locals (LocalBool :type Boolean) (LocalIndex :type Integer))
  (for (_array_element _array_index) (`self.Slots`)
    (if (not (`KismetSystemLibrary.IsValidClass` (`.ItemClass_2_701FE76C4B15DAF086A2F4B6B79A8CF2` (break `/Game/Blueprints/Structures/InventoryStruct` _array_element))))
      (set `local.LocalBool` true)
      (set `local.LocalIndex` _array_index)
      (break)))
  (return (`local.LocalBool`) (`local.LocalIndex`)))

(fn `SearchFreeStack`
  (params (ItemClass :type "/Game/Blueprints/Items/BP_BasePickUp Class Reference"))
  (returns (Succuss :type Boolean) (Index :type Integer))
  (locals (LocalBool :type Boolean) (LocalIndex :type Integer))
  (for (_array_element _array_index) (`self.Slots`)
    (bind (_itemclass _quantity) (break `/Game/Blueprints/Structures/InventoryStruct` _array_element))
    (if (`KismetSystemLibrary.IsValidClass` _itemclass)
      (if (and (== _itemclass ItemClass) (<= _quantity (`self.MaxStackSize`)))
        (set `local.LocalBool` false)
        (set `local.LocalIndex` _array_index)
        (break))))
  (return (`local.LocalBool`) (`local.LocalIndex`)))

(fn `UseItem`
  (bind (_output_itemclass _output_quantity) (break `/Game/Blueprints/Structures/InventoryStruct` (`|GetArrayItem` (`self.Slots`) (`self.CurrentItemIndex`))))
  (if (`KismetSystemLibrary.IsValidClass` _output_itemclass)
    (bind _returnvalue (`|SpawnActorFromClass` _output_itemclass (`KismetMathLibrary.MakeTransform` (0.0 0.0 0.0)) "Undefined" "OverrideRootScale" null null))
    (bind _item_was_used (`/Game/Blueprints/Items/BP_BasePickUp.UseItem` _returnvalue (`self.PlayerRef`)))
    (if _item_was_used
      (`Actor.K2_DestroyActor` _returnvalue)
      (bind _result (`/Engine/EditorBlueprintResources/StandardMacros.DecrementInt` _output_quantity)
        (:`  `
          (if (<= _result 0)
            (`KismetArrayLibrary.Array_Set` (`self.Slots`) (`self.CurrentItemIndex`) (make `/Game/Blueprints/Structures/InventoryStruct` null))
            (`self.CycleItemNext`)))))))