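; Foot IK component that plants a standing character's feet on uneven ground, easing offsets back to neutral while moving.
; Each tick when idle, downward traces at both foot sockets yield height offsets and surface-aligned rotations.
; The lower foot drives pelvis drop and capsule half-height shrink, with interpolated values sent to the AnimInstance through interface messages.
; Disabling snaps AnimInstance values to zero; a gate-based variant for static ground is left unwired from Tick.
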(event `self.ReceiveTick`
  (params (DeltaSeconds :type "Float (single-precision)"))
  (bind _isenabled (`self.IsEnabled`))
  (if _isenabled
    (if (and _isenabled (`self.IsMoving`))
      (`self.IKResetVarsInterp`)
      (else
        (`self.IKupdate`)))
    (else
      (`self.IKResetVarsSnap`))))

(event `EnableIK`
  ;[1 1 1] a more optomized version for when the ground never moves
  (`/Engine/EditorBlueprintResources/StandardMacros.Gate` true :!via `Open` :!label _label
    (:`Exit`
      (`self.IKUpdate`))))

(event `DisableIK`
  ;[1 1 1] a more optomized version for when the ground never moves
  (`KismetSystemLibrary.Delay` (`self.IKTimeout`))
  (goto _label :!via `Close`))

(fn `IKFootTrace`
  (params (TraceDistance :type "Float (double-precision)") (SocketName :type Name))
  (returns (Offset :type "Float (double-precision)") (Impact :type "Vector Structure"))
  (locals (Distance :type "Float (double-precision)") (Socket :type Name))
  (bind (_returnvalue_x _returnvalue_y _returnvalue_z) (`KismetMathLibrary.BreakVector` (`Actor.K2_GetActorLocation` (`self.GetOwner`))))
  (bind _x (.x (`SceneComponent.GetSocketLocation` (`self.Mesh`) (`local.Socket`))))
  (bind _y (.y (`SceneComponent.GetSocketLocation` (`self.Mesh`) (`local.Socket`))))
  (set `local.Distance` TraceDistance)
  (set `local.Socket` SocketName)
  (bind (_outhit _returnvalue) (`KismetSystemLibrary.LineTraceSingle` (`KismetMathLibrary.MakeVector` _x _y _returnvalue_z) (`KismetMathLibrary.MakeVector` _x _y (- (- _returnvalue_z (`self.IKCapsuleHalfHeight`)) (`local.Distance`))) "TraceTypeQuery1"))
  (bind (_bblockinghit _binitialoverlap _time _distance _location _impactpoint _normal _impactnormal _physmat _hitactor _hitcomponent _hitbonename _hititem _faceindex _tracestart _traceend) (`GameplayStatics.BreakHitResult` _outhit))
  (return (`KismetMathLibrary.SelectFloat` (+ (- (`KismetMathLibrary.VSize` (- _location _traceend)) (`local.Distance`)) (`self.IKAdjustOffset`)) 0.0 _returnvalue) _impactnormal))

(fn `IKResetVarsInterp`
  (bind _animinstance (`self.AnimInstance`))
  (bind _animinstance_2 (`self.AnimInstance`))
  (bind _animinstance_3 (`self.AnimInstance`))
  (`|ExecutionSequence`
    (:`then_0`
      (bind _righteffectorlocation (message `/Game/Blueprints/Interfaces/BI_IKAnimation.GetRightEffectorLocation_BI` _animinstance_2))
      (bind _returnvalue (`self.IKUpdateFootOffset` 0.0 _righteffectorlocation (`self.IKFeetInterpSpeed`)))
      (message `/Game/Blueprints/Interfaces/BI_IKAnimation.SetRightEffectorLocation_BI` _animinstance_2 _returnvalue)
      (bind _lefteffectorlocation (message `/Game/Blueprints/Interfaces/BI_IKAnimation.GetLeftEffectorLocation_BI` _animinstance_2))
      (bind _returnvalue_2 (`self.IKUpdateFootOffset` 0.0 _lefteffectorlocation (`self.IKFeetInterpSpeed`)))
      (message `/Game/Blueprints/Interfaces/BI_IKAnimation.SetLeftEffectorLocation_BI` _animinstance_2 _returnvalue_2))
    (:`then_1`
      (bind _rotation (message `/Game/Blueprints/Interfaces/BI_IKAnimation.GetRightFootRotation_BI` _animinstance_3))
      (bind _returnvalue_3 (`self.IKUpdateFootRotation` (struct) _rotation (`self.IKFeetInterpSpeed`)))
      (message `/Game/Blueprints/Interfaces/BI_IKAnimation.SetRightFootRotation_BI` _animinstance_3 _returnvalue_3)
      (bind _rotation_2 (message `/Game/Blueprints/Interfaces/BI_IKAnimation.GetLeftFootRotation_BI` _animinstance_3))
      (bind _returnvalue_4 (`self.IKUpdateFootRotation` (struct) _rotation_2 (`self.IKFeetInterpSpeed`)))
      (message `/Game/Blueprints/Interfaces/BI_IKAnimation.SetLeftFootRotation_BI` _animinstance_3 _returnvalue_4))
    (:`then_2`
      (bind _pelvisoffset (message `/Game/Blueprints/Interfaces/BI_IKAnimation.GetPelvisOffset_BI` _animinstance))
      (bind _returnvalue_5 (`self.IKUpdateFootOffset` 0.0 _pelvisoffset (`self.IKPelvisInterpSpeed`)))
      (message `/Game/Blueprints/Interfaces/BI_IKAnimation.SetPelvisOffset_BI` _animinstance _returnvalue_5)
      (`self.UpdateCapsuleHalfHeight` 0.0 true))))

(fn `IKResetVarsSnap`
  (bind _animinstance (`self.AnimInstance`))
  (bind _animinstance_2 (`self.AnimInstance`))
  (`|ExecutionSequence`
    (:`then_0`
      (message `/Game/Blueprints/Interfaces/BI_IKAnimation.SetRightEffectorLocation_BI` _animinstance 0.0)
      (message `/Game/Blueprints/Interfaces/BI_IKAnimation.SetLeftEffectorLocation_BI` _animinstance 0.0))
    (:`then_1`
      (message `/Game/Blueprints/Interfaces/BI_IKAnimation.SetRightFootRotation_BI` _animinstance_2 (struct))
      (message `/Game/Blueprints/Interfaces/BI_IKAnimation.SetLeftFootRotation_BI` _animinstance_2 (struct)))
    (:`then_2`
      (message `/Game/Blueprints/Interfaces/BI_IKAnimation.SetPelvisOffset_BI` (`self.AnimInstance`) 0.0))))

(fn `IKUpdate`
  (locals (LeftFootOffset :type "Float (double-precision)" :default 0.0) (RightFootOffset :type "Float (double-precision)" :default 0.0) (PelvisOffset :type "Float (double-precision)" :default 0.0))
  (bind _animinstance (`self.AnimInstance`))
  (bind _animinstance_2 (`self.AnimInstance`))
  (bind _animinstance_3 (`self.AnimInstance`))
  (bind _animinstance_4 (`self.AnimInstance`))
  (bind _returnvalue (`KismetMathLibrary.FMin` (`local.LeftFootOffset`) (`local.RightFootOffset`)))
  (`|ExecutionSequence`
    (:`then_0`
      ;[1 1 1] calculate feet offset and rotation
      (bind (_offset _impact) (`self.IKFootTrace` (`self.IKTraceDistance`) (`self.IKLeftFootSocket`)))
      (set `local.LeftFootOffset` _offset)
      (bind _rotation (message `/Game/Blueprints/Interfaces/BI_IKAnimation.GetLeftFootRotation_BI` _animinstance_4))
      (bind _returnvalue_2 (`self.IKUpdateFootRotation` (`self.NormalToRotator` _impact) _rotation (`self.IKFeetInterpSpeed`)))
      (message `/Game/Blueprints/Interfaces/BI_IKAnimation.SetLeftFootRotation_BI` _animinstance_4 _returnvalue_2))
    (:`then_1`
      (bind (_offset_2 _impact_2) (`self.IKFootTrace` (`self.IKTraceDistance`) (`self.IKRightFootSocket`)))
      (set `local.RightFootOffset` _offset_2)
      (bind _rotation_2 (message `/Game/Blueprints/Interfaces/BI_IKAnimation.GetRightFootRotation_BI` _animinstance_2))
      (bind _returnvalue_3 (`self.IKUpdateFootRotation` (`self.NormalToRotator` _impact_2) _rotation_2 (`self.IKFeetInterpSpeed`)))
      (message `/Game/Blueprints/Interfaces/BI_IKAnimation.SetRightFootRotation_BI` _animinstance_2 _returnvalue_3))
    (:`then_2`
      ;[1 1 1] update the pelvis location
      (bind _output_get (set `local.PelvisOffset` (`KismetMathLibrary.SelectFloat` _returnvalue 0.0 (< _returnvalue 0.0))))
      (bind _pelvisoffset (message `/Game/Blueprints/Interfaces/BI_IKAnimation.GetPelvisOffset_BI` _animinstance))
      (bind _returnvalue_4 (`self.IKUpdateFootOffset` _output_get _pelvisoffset (`self.IKPelvisInterpSpeed`)))
      (message `/Game/Blueprints/Interfaces/BI_IKAnimation.SetPelvisOffset_BI` _animinstance _returnvalue_4)
      (`self.UpdateCapsuleHalfHeight` (`local.PelvisOffset`)))
    (:`then_3`
      ;[1 1 1] Update the location of both feet
      (bind _lefteffectorlocation (message `/Game/Blueprints/Interfaces/BI_IKAnimation.GetLeftEffectorLocation_BI` (`self.AnimInstance`)))
      (bind _returnvalue_5 (`self.IKUpdateFootOffset` (- (`local.LEftFootOffset`) (`local.PelvisOffset`)) _lefteffectorlocation (`self.IKFeetInterpSpeed`)))
      (message `/Game/Blueprints/Interfaces/BI_IKAnimation.SetLeftEffectorLocation_BI` _animinstance_3 _returnvalue_5)
      (bind _righteffectorlocation (message `/Game/Blueprints/Interfaces/BI_IKAnimation.GetRightEffectorLocation_BI` _animinstance_3))
      (bind _returnvalue_6 (`self.IKUpdateFootOffset` (- (`local.RightFootOffset`) (`local.PelvisOffset`)) _righteffectorlocation (`self.IKFeetInterpSpeed`)))
      (message `/Game/Blueprints/Interfaces/BI_IKAnimation.SetRightEffectorLocation_BI` _animinstance_3 _returnvalue_6))
    (:`then_4`
      ;[1 1 1] Disable IK when it has reached the desired state
      (bind _lefteffectorlocation_2 (message `/Game/Blueprints/Interfaces/BI_IKAnimation.GetLeftEffectorLocation_BI` (`self.AnimInstance`)))
      (bind _righteffectorlocation_2 (message `/Game/Blueprints/Interfaces/BI_IKAnimation.GetRightEffectorLocation_BI` (`self.AnimInstance`)))
      (if (and (`KismetMathLibrary.NearlyEqual_FloatFloat` _lefteffectorlocation_2 (- (`local.LEftFootOffset`) (`local.PelvisOffset`)) 1.0) (`KismetMathLibrary.NearlyEqual_FloatFloat` _righteffectorlocation_2 (- (`local.RightFootOffset`) (`local.PelvisOffset`)) 1.0))
        (`self.DisableIK`)))))

(fn `IKUpdateFootOffset`
  (params (`Target Value` :type "Float (double-precision)") (EffectorValue :type "Float (double-precision) (by ref)") (InterpSpeed :type "Float (double-precision)"))
  (returns (ReturnValue :type "Float (double-precision)"))
  (locals (Target :type "Float (double-precision)"))
  (set `local.Target` `Target Value`)
  (return (`KismetMathLibrary.FInterpTo` EffectorValue (`local.Target`) (`GameplayStatics.GetWorldDeltaSeconds`) InterpSpeed)))

(fn `IKUpdateFootRotation`
  (params (TargetValue :type "Rotator Structure") (RotationVar :type "Rotator Structure (by ref)") (IKFeetInterpSpeed :type "Float (double-precision)"))
  (returns (ReturnValue :type "Rotator Structure"))
  (locals (Target :type "Rotator Structure"))
  (set `local.Target` TargetValue)
  (return (`KismetMathLibrary.RInterpTo` RotationVar TargetValue (`GameplayStatics.GetWorldDeltaSeconds`) IKFeetInterpSpeed)))

(fn `Initialize`
  (params (CapsuleComponent :type "CapsuleComponent Object Reference") (Mesh :type "SkeletalMeshComponent Object Reference"))
  (bind _output_get (set `self.CapsuleComponent` CapsuleComponent))
  (set `self.IKCapsuleHalfHeight` (`CapsuleComponent.GetScaledCapsuleHalfHeight` _output_get))
  (bind _output_get_2 (set `self.Mesh` Mesh))
  (set `self.AnimInstance` (`SkeletalMeshComponent.GetAnimInstance` _output_get_2))
  (set `self.IsEnabled` true))

(fn `IsMoving`
  (returns (IsMoving :type Boolean))
  ;[1 1 1] Pure function to check if the character is moving or not
  (return (> (`KismetMathLibrary.VSize` (`Actor.GetVelocity` (`self.GetOwner`))) 0.0)))

(fn `NormalToRotator`
  (params (Normal :type "Vector Structure"))
  (returns (Rotator :type "Rotator Structure"))
  (bind _z (.z Normal))
  (return (`KismetMathLibrary.MakeRotator` (`KismetMathLibrary.DegAtan2` (.y Normal) _z) (* (`KismetMathLibrary.DegAtan2` (.x Normal) _z) -1.0))))

(fn `UpdateCapsuleHalfHeight`
  (params (PelvisOffset :type "Float (double-precision)") (ResetDefault :type Boolean))
  (bind _capsulecomponent (`self.CapsuleComponent`))
  (`CapsuleComponent.SetCapsuleHalfHeight` _capsulecomponent (`KismetMathLibrary.FInterpTo` (`CapsuleComponent.GetScaledCapsuleHalfHeight` _capsulecomponent) (`KismetMathLibrary.SelectFloat` (`self.IKCapsuleHalfHeight`) (- (`self.IKCapsuleHalfHeight`) (/ (`KismetMathLibrary.Abs` PelvisOffset) 2.0)) ResetDefault) (`GameplayStatics.GetWorldDeltaSeconds`) (`self.IKPelvisInterpSpeed`)) true))