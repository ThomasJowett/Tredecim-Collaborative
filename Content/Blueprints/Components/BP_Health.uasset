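; Health component that gives its owner segmented health with delayed regeneration up to the current segment's cap.
; BeginPlay fills health from segment count times HP per segment, and each hit lowers it, pauses regen and removes at most one segment when a boundary is reached.
; A restarted delay timer starts a looping regen tick that stops at the remaining segments' total.
; Health at or below the minimum sends a Die interface message to the owner.
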(event `TakeDamage`
  (params (Damage :type "Float (double-precision)"))
  ;[1 1 1] Take Damage
  (set `self.CanRegen` false)
  (bind _output_get (set `self.CurrentHealth` (- (`self.CurrentHealth`) Damage)))
  (`self.SegmentCheck`)
  (`KismetSystemLibrary.K2_SetTimerDelegate` (delegate `HealDelay`) 2.0)
  (if (<= _output_get (`self.MinHealth`))
    (message `/Game/Blueprints/Interfaces/BI_Death.Die_BI` (`self.GetOwner`))))

(event `HealDelay`
  ;[1 1 1] Take Damage
  (set `self.CanRegen` true)
  (`KismetSystemLibrary.K2_SetTimer` null "RegenHealth" 0.02 true))

(event `self.ReceiveBeginPlay`
  (bind _maxsegmentamt (`self.MaxSegmentAmt`))
  ;[1 1 1] Set HP with base segment amount
  (set `self.CurrentSegmentAmt` _maxsegmentamt)
  (bind _output_get (set `self.MaxHealth` (* _maxsegmentamt (`self.HPPerSegment`))))
  (set `self.CurrentHealth` _output_get))

(event `RegenHealth`
  ;[1 1 1] Auto Heal segment
  (if (`self.CanRegen`)
    (if (< (`self.CurrentHealth`) (* (`self.CurrentSegmentAmt`) (`self.HPPerSegment`)))
      (set `self.CurrentHealth` (+ (`self.CurrentHealth`) (* 0.02 (`self.HealthRegenRate`))))
      (else
        (set `self.CanRegen` false)
        (`KismetSystemLibrary.K2_ClearTimer` null "RegenHealth")))))

(event `SegmentCheck`
  (bind _returnvalue (- (`self.CurrentSegmentAmt`) 1))
  ;[1 1 1] HP Segement check
  (if (<= (`self.CurrentHealth`) (* _returnvalue (`self.HPPerSegment`)))
    (set `self.CurrentSegmentAmt` _returnvalue)))