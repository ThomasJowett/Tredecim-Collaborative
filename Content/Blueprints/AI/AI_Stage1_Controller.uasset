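; AI controller for the Stage 1 boss that runs its behavior tree and stores the player character in the blackboard.
; On BeginPlay it finds the first CH_ThirdPerson and binds its death event to clear the reference, which GetTarget exposes.
; SetPlayerDistance buckets player distance by melee and ranged thresholds into the RangeToPlayer key, printing the result.
; The looping timer meant to drive that check is disconnected and never runs.
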(event `self.ReceiveBeginPlay`
  (bind _returnvalue (`AIBlueprintHelperLibrary.GetBlackboard` null))
  ;[1 1 1] Begin play
  (`self.RunBehaviorTree` "/Game/Blueprints/AI/Stage_01_Boss_BT.Stage_01_Boss_BT")
  (`self.UseBlackboard` "/Game/Blueprints/AI/Boss_Blackboard.Boss_Blackboard")
  (bind _outactors (`GameplayStatics.GetAllActorsOfClass` "/Game/Blueprints/CH_ThirdPerson.CH_ThirdPerson_C"))
  (bind _output_get (set `self.PlayerRef` (`|GetArrayItem` _outactors)))
  (add `/Game/Blueprints/CH_ThirdPerson.PlayerDeath` _output_get (delegate `PlayerIsDead`))
  (`/Engine/EditorBlueprintResources/StandardMacros.IsValid` _returnvalue
    (:`Is Valid`
      (`BlackboardComponent.SetValueAsObject` _returnvalue (`KismetSystemLibrary.MakeLiteralName` (`self.Player`)) _output_get))))

(event `PlayerIsDead`
  (set `self.PlayerRef` null))

(event `AttackTimer`
  (`self.SetPlayerDistance`))

(fn `GetTarget`
  (returns (Target :type "Actor Object Reference"))
  (return (`self.PlayerRef`)))

(fn `SetPlayerDistance`
  (locals (RangeType :type "/Game/Blueprints/AI/Enums/E_RangeStates Enum" :default "NewEnumerator0"))
  (bind _returnvalue (`AIBlueprintHelperLibrary.GetBlackboard` null))
  (bind _playerref (`self.PlayerRef`))
  (bind _rangetype (`local.RangeType`))
  (bind _returnvalue_2 (`self.GetDistanceTo` _playerref (`self.K2_GetPawn`)))
  (`/Engine/EditorBlueprintResources/StandardMacros.IsValid` _playerref
    (:`Is Valid`
      (if (<= _returnvalue_2 (`self.MeleeAttackDistance`))
        (set `local.RangeType` "NewEnumerator0")
        (elif (> _returnvalue_2 (`self.RangedAttackDistance`))
          (set `local.RangeType` "NewEnumerator1")
          (else
            (set `local.RangeType` "NewEnumerator2"))))
      (`/Engine/EditorBlueprintResources/StandardMacros.IsValid` _returnvalue
        (:`Is Valid`
          (`KismetSystemLibrary.PrintString` (`|GetEnumeratorNameAsString` _rangetype))
          (`BlackboardComponent.SetValueAsEnum` _returnvalue (`KismetSystemLibrary.MakeLiteralName` (`self.RangeToPlayer`)) _rangetype))))))

(fn `UserConstructionScript`)