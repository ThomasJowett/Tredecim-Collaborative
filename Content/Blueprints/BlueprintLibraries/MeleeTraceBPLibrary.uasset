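; Blueprint function library providing MeleeTrace, a melee hit check along a line segment with optional debug drawing.
; World mode runs a channel line trace and can report no hit when it strikes a Character.
; Otherwise it scans all Characters within a given distance of the instigator, excluding itself, and line traces directly against each skeletal mesh component, returning the first hit found rather than the nearest.
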(fn `MeleeTrace`
  (params (Instigator :type "Character Object Reference") (Distance :type "Float (double-precision)") (StartLocation :type "Vector Structure") (EndLocation :type "Vector Structure") (DrawTrace :type Boolean) (TraceAgainstWorld :type Boolean) (WorldTraceChannel :type "ETraceTypeQuery Enum" :default "TraceTypeQuery1") (WorldIgnoreCharacters :type Boolean) (LineColour :type "LinearColor Structure") (DrawTime :type "Float (double-precision)"))
  (returns (HitResult :type "HitResult Structure") (HasHit :type Boolean))
  (locals (CollisionQueryParameters :type Boolean))
  (`/Engine/EditorBlueprintResources/StandardMacros.IsValid` Instigator
    (:`Is Valid`
      (if DrawTrace
        (`KismetSystemLibrary.DrawDebugLine` Instigator StartLocation EndLocation LineColour DrawTime 1.0))
      (if TraceAgainstWorld
        (bind (_outhit _returnvalue) (`KismetSystemLibrary.LineTraceSingle` Instigator StartLocation EndLocation WorldTraceChannel))
        (if WorldIgnoreCharacters
          (cast `Character` (`.HitActor` (`GameplayStatics.BreakHitResult` _outhit))
            (:`then`
              (return (struct) false))
            (:`CastFailed`
              _)))
        (return _outhit _returnvalue)
        (else
          (bind _outactors (`GameplayStatics.GetAllActorsOfClass` null "/Script/Engine.Character"))
          (for _array_element _outactors
            (if (!= Instigator _array_element)
              (if (<= (`Actor.GetDistanceTo` Instigator _array_element) Distance)
                (bind _ascharacter (cast `Character` _array_element))
                (bind (_hitlocation _hitnormal _bonename _outhit_2 _returnvalue_2) (`PrimitiveComponent.K2_LineTraceComponent` (`Character.Mesh` _ascharacter) StartLocation EndLocation true false))
                (if _returnvalue_2
                  (return _outhit_2 _returnvalue_2)))))
          (return (struct) false))))
    (:`Is Not Valid`
      (return (struct) false))))