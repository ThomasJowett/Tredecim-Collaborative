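; BP_BuffStall is a vending-cart stall that grants a timed speed, damage or health-regen buff on overlap.
; The construction script sets particle circle and cart material from BuffType, including a Range type that only gets a message on overlap.
; Overlap sends ApplyBuffsMessage, adds to CH_ThirdPerson walk speeds, equipped-weapon damage or regen rate, then subtracts after a Delay.
; Per-stall active flags block stacking, and damage undo targets whichever weapon is then equipped.
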(event `self.ReceiveActorBeginOverlap`
  (params (OtherActor :type "Actor Object Reference"))
  (bind _buffduration (`self.BuffDuration`))
  (bind _buff_type (`self.buff Type`))
  ;[0.02247 1 0] Comment
  (message `/Game/Blueprints/Interfaces/BI_Buff.Apply Buffs` OtherActor _buff_type _buffduration)
  (switch `/Game/Blueprints/Enumerations/E_Buff` _buff_type
    (:`NewEnumerator1`
      (`self.SpeedBuff` OtherActor)
      (`KismetSystemLibrary.Delay` _buffduration)
      (`self.UndoSpeed` OtherActor))
    (:`NewEnumerator2`
      (`self.DamageBuff` OtherActor)
      (`KismetSystemLibrary.Delay` _buffduration)
      (`self.UndoDamage` OtherActor))
    (:`NewEnumerator3`
      (`self.RegenBuff` OtherActor)
      (`KismetSystemLibrary.Delay` _buffduration)
      (`self.UndoRegen` OtherActor))))

(fn `DamageBuff`
  (params (PlayerChar :type "Actor Object Reference"))
  (bind _damagebuffamt (`self.DamageBuffAmt`))
  ;[0.02247 1 0] Damage Buff
  (if (not (`self.DamageIsActive`))
    (bind _asch_third_person (cast `/Game/Blueprints/CH_ThirdPerson` PlayerChar))
    (bind _equippedweapon (`/Game/Blueprints/Components/BP_WeaponInventory.GetEquippedWeapon` (`/Game/Blueprints/CH_ThirdPerson.WeaponInventory` _asch_third_person)))
    (set `/Game/Weapons/WP_BaseWeapon.LightDamage` (+ (`/Game/Weapons/WP_BaseWeapon.LightDamage` _equippedweapon) _damagebuffamt) _equippedweapon)
    (set `/Game/Weapons/WP_BaseWeapon.HeavyDamage` (+ _damagebuffamt (`/Game/Weapons/WP_BaseWeapon.HeavyDamage` _equippedweapon)) _equippedweapon)
    (set `self.DamageIsActive` true)))

(fn `RegenBuff`
  (params (PlayerChar :type "Actor Object Reference"))
  ;[0 1 0.03599] Regen Buff
  (if (not (`self.RegenIsActive`))
    (bind _asch_third_person (cast `/Game/Blueprints/CH_ThirdPerson` PlayerChar))
    (bind _health (`/Game/Blueprints/CH_ThirdPerson.Health` _asch_third_person))
    (set `/Game/Blueprints/Components/BP_Health.HealthRegenRate` (+ (`self.RegenBuffAmt`) (`/Game/Blueprints/Components/BP_Health.HealthRegenRate` _health)) _health)
    (set `self.RegenIsActive` true)))

(fn `SpeedBuff`
  (params (PlayerChar :type "Actor Object Reference"))
  (bind _walkspeedbuffamt (`self.WalkSpeedBuffAmt`))
  ;[0 1 0.03342] Change Player Speed
  (if (not (`self.SpeedIsActive`))
    (bind _asch_third_person (cast `/Game/Blueprints/CH_ThirdPerson` PlayerChar))
    (set `/Game/Blueprints/CH_ThirdPerson.DefaultWalkSpeed` (+ (`/Game/Blueprints/CH_ThirdPerson.DefaultWalkSpeed` _asch_third_person) _walkspeedbuffamt) _asch_third_person)
    (set `/Game/Blueprints/CH_ThirdPerson.CombatWalkSpeed` (+ (`/Game/Blueprints/CH_ThirdPerson.CombatWalkSpeed` _asch_third_person) _walkspeedbuffamt) _asch_third_person)
    (set `/Game/Blueprints/CH_ThirdPerson.BlockingWalkSpeed` (+ (`/Game/Blueprints/CH_ThirdPerson.BlockingWalkSpeed` _asch_third_person) _walkspeedbuffamt) _asch_third_person)
    (set `self.SpeedIsActive` true)))

(fn `UndoDamage`
  (params (`Player Char` :type "Actor Object Reference"))
  (bind _damagebuffamt (`self.DamageBuffAmt`))
  ;[0.02247 1 0] Damage Buff
  (if (`self.DamageIsActive`)
    (bind _asch_third_person (cast `/Game/Blueprints/CH_ThirdPerson` `Player Char`))
    (bind _equippedweapon (`/Game/Blueprints/Components/BP_WeaponInventory.GetEquippedWeapon` (`/Game/Blueprints/CH_ThirdPerson.WeaponInventory` _asch_third_person)))
    (set `/Game/Weapons/WP_BaseWeapon.LightDamage` (- (`/Game/Weapons/WP_BaseWeapon.LightDamage` _equippedweapon) _damagebuffamt) _equippedweapon)
    (set `/Game/Weapons/WP_BaseWeapon.HeavyDamage` (- (`/Game/Weapons/WP_BaseWeapon.HeavyDamage` _equippedweapon) _damagebuffamt) _equippedweapon)
    (set `self.DamageIsActive` false)))

(fn `UndoRegen`
  (params (PlayerChar :type "Actor Object Reference"))
  ;[0 1 0.03599] Regen Buff
  (if (`self.RegenIsActive`)
    (bind _asch_third_person (cast `/Game/Blueprints/CH_ThirdPerson` PlayerChar))
    (bind _health (`/Game/Blueprints/CH_ThirdPerson.Health` _asch_third_person))
    (set `/Game/Blueprints/Components/BP_Health.HealthRegenRate` (- (`/Game/Blueprints/Components/BP_Health.HealthRegenRate` _health) (`self.RegenBuffAmt`)) _health)
    (set `self.RegenIsActive` false)))

(fn `UndoSpeed`
  (params (`Player Char` :type "Actor Object Reference"))
  (bind _walkspeedbuffamt (`self.WalkSpeedBuffAmt`))
  ;[0 1 0.03342] Change Player Speed
  (if (`self.SpeedIsActive`)
    (bind _asch_third_person (cast `/Game/Blueprints/CH_ThirdPerson` `Player Char`))
    (set `/Game/Blueprints/CH_ThirdPerson.DefaultWalkSpeed` (- (`/Game/Blueprints/CH_ThirdPerson.DefaultWalkSpeed` _asch_third_person) _walkspeedbuffamt) _asch_third_person)
    (set `/Game/Blueprints/CH_ThirdPerson.CombatWalkSpeed` (- (`/Game/Blueprints/CH_ThirdPerson.CombatWalkSpeed` _asch_third_person) _walkspeedbuffamt) _asch_third_person)
    (set `/Game/Blueprints/CH_ThirdPerson.BlockingWalkSpeed` (- (`/Game/Blueprints/CH_ThirdPerson.BlockingWalkSpeed` _asch_third_person) _walkspeedbuffamt) _asch_third_person)
    (set `self.SpeedIsActive` false)))

(fn `UserConstructionScript`
  (bind _buff_circle (`self.Buff_Circle`))
  (bind _sm_vendingcart (`self.SM_VendingCart`))
  (switch `/Game/Blueprints/Enumerations/E_Buff` (`self.buff Type`)
    (:`NewEnumerator0`
      (`ParticleSystemComponent.SetTemplate` _buff_circle "/Game/RyanFX/Buffs/Range/Range_Buff_Circle_P.Range_Buff_Circle_P")
      (`PrimitiveComponent.SetMaterial` _sm_vendingcart 2 "/Game/Ben_DevMaterials/Dev_master_Purple.Dev_master_Purple"))
    (:`NewEnumerator1`
      (`ParticleSystemComponent.SetTemplate` _buff_circle "/Game/RyanFX/Buffs/Speed/Speed_Buff_Circle_P.Speed_Buff_Circle_P")
      (`PrimitiveComponent.SetMaterial` _sm_vendingcart 2 "/Game/Ben_DevMaterials/Dev_master_Darkblue.Dev_master_Darkblue"))
    (:`NewEnumerator2`
      (`ParticleSystemComponent.SetTemplate` _buff_circle "/Game/RyanFX/Buffs/Attack/Attack_Buff_Circle_P1.Attack_Buff_Circle_P1")
      (`PrimitiveComponent.SetMaterial` _sm_vendingcart 2 "/Game/Materials/M_PlasterRed.M_PlasterRed"))
    (:`NewEnumerator3`
      (`ParticleSystemComponent.SetTemplate` _buff_circle "/Game/RyanFX/Buffs/Health/HealthBuff_Circle_P.HealthBuff_Circle_P")
      (`PrimitiveComponent.SetMaterial` _sm_vendingcart 2 "/Game/Ben_DevMaterials/Dev_master_Grass.Dev_master_Grass"))))