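; HUD_Main is the game's main HUD Blueprint, creating the UI_HUDLayout widget on begin play and adding it to the viewport.
; BI-suffixed events relay pause, buff activation and boss health changes to the layout's child widgets.
; Pause calls ShowScreen, then a FlipFlop alternately hides or restores health and buff widgets while switching input mode and mouse cursor.
; Buff events route range, speed, power and health regen to two buff widgets.
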(event `self.ReceiveBeginPlay`
  ;[1 1 1] Begin Play
  (bind _returnvalue (`|CreateWidget` "/Game/UI/Widgets/UI_HUDLayout.UI_HUDLayout_C" (`GameplayStatics.GetPlayerController` 0)))
  (bind _output_get (set `self.HUDWidget` _returnvalue))
  (`UserWidget.AddToViewport` _output_get 0))

(event `/Game/Blueprints/Interfaces/BI_UI.Pause_BI`
  (bind _returnvalue (`GameplayStatics.GetPlayerController` 0))
  (bind _hudwidget (`self.HUDWidget`))
  ;[1 1 1] Pause
  (`/Game/UI/Widgets/UI_Pause.ShowScreen` (`/Game/UI/Widgets/UI_HUDLayout.UI_Pause` _hudwidget) self)
  (`/Engine/EditorBlueprintResources/StandardMacros.FlipFlop`
    (:`A`
      (`Widget.SetVisibility` (`/Game/UI/Widgets/UI_HUDLayout.UI_BossHealth` _hudwidget) "Hidden")
      (`Widget.SetVisibility` (`/Game/UI/Widgets/UI_HUDLayout.UI_Health` _hudwidget) "Hidden")
      (`Widget.SetVisibility` (`/Game/UI/Widgets/UI_HUDLayout.UI_Buffs_1` _hudwidget) "Hidden")
      (`Widget.SetVisibility` (`/Game/UI/Widgets/UI_HUDLayout.UI_Buffs_2` _hudwidget) "Hidden")
      (`WidgetBlueprintLibrary.SetInputMode_GameAndUIEx` _returnvalue null)
      (set `PlayerController.bShowMouseCursor` true _returnvalue))
    (:`B`
      (`Widget.SetVisibility` (`/Game/UI/Widgets/UI_HUDLayout.UI_Buffs_2` _hudwidget) "Visible")
      (`Widget.SetVisibility` (`/Game/UI/Widgets/UI_HUDLayout.UI_BossHealth` _hudwidget) "Visible")
      (`Widget.SetVisibility` (`/Game/UI/Widgets/UI_HUDLayout.UI_Health` _hudwidget) "Visible")
      (`Widget.SetVisibility` (`/Game/UI/Widgets/UI_HUDLayout.UI_Buffs_1` _hudwidget) "Visible")
      (`WidgetBlueprintLibrary.SetInputMode_GameOnly` _returnvalue)
      (set `PlayerController.bShowMouseCursor` false _returnvalue))))

(event `/Game/Blueprints/Interfaces/BI_UI.Buff_BI`
  (params (`Buff Index` :type "/Game/Blueprints/Enumerations/E_Buff Enum" :default "NewEnumerator0"))
  (bind _hudwidget (`self.HUDWidget`))
  (bind _ui_buffs_1 (`/Game/UI/Widgets/UI_HUDLayout.UI_Buffs_1` _hudwidget))
  (bind _ui_buffs_2 (`/Game/UI/Widgets/UI_HUDLayout.UI_Buffs_2` _hudwidget))
  ;[1 1 1] Buffs
  (switch `/Game/Blueprints/Enumerations/E_Buff` `Buff Index`
    (:`NewEnumerator0`
      (`/Game/UI/Widgets/UI_Buffs_2.RangeBuffActive` _ui_buffs_2))
    (:`NewEnumerator1`
      (`/Game/UI/Widgets/UI_Buffs_1.SpeedBuffActive` _ui_buffs_1))
    (:`NewEnumerator2`
      (`/Game/UI/Widgets/UI_Buffs_1.PowerBuffActive` _ui_buffs_1))
    (:`NewEnumerator3`
      (`/Game/UI/Widgets/UI_Buffs_2.HealthBuffActive` _ui_buffs_2))))

(event `/Game/Blueprints/Interfaces/BI_UI.BossHealth_BI`
  (params (MaxHealth :type "Float (single-precision)") (CurrentHealth :type "Float (single-precision)"))
  (`/Game/UI/Widgets/UI_BossHealth.Damaged` (`/Game/UI/Widgets/UI_HUDLayout.UI_BossHealth` (`self.HUDWidget`)) MaxHealth CurrentHealth))

(fn `UserConstructionScript`)