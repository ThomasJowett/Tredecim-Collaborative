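; BP_StreamVolume is a trigger box that streams levels in and out as the player character enters it.
; On overlap it first unloads the LevelToUnLoad level if loaded, then loads and shows the LevelToLoad level if not already loaded.
; Either name can be None to skip that step, both operations are non-blocking, and each prints an on-screen debug message.
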(event `self.Box.OnComponentBeginOverlap`
  (params (OverlappedComponent :type "PrimitiveComponent Object Reference") (OtherActor :type "Actor Object Reference") (OtherComp :type "PrimitiveComponent Object Reference") (OtherBodyIndex :type Integer) (bFromSweep :type Boolean) (SweepResult :type "HitResult Structure (by ref)"))
  (bind _leveltoload (`self.LevelToLoad`))
  (bind _leveltounload (`self.LevelToUnLoad`))
  ;[0.1212 1 0.02061] Comment
  (if (== OtherActor (`GameplayStatics.GetPlayerCharacter` 0))
    (`|ExecutionSequence`
      (:`then_0`
        (if (== _leveltounload "None")
          _
          (elif (`LevelStreaming.IsLevelLoaded` (`GameplayStatics.GetStreamingLevel` _leveltounload))
            (`GameplayStatics.UnloadStreamLevel` _leveltounload)
            (`KismetSystemLibrary.PrintString` (`KismetStringLibrary.Concat_StrStr` (`KismetStringLibrary.Conv_NameToString` _leveltounload) "UnLoaded") true true (struct :`R` 1.0 :`G` 0.03977 :`B` 0.009923 :`A` 1.0)))))
      (:`then_1`
        (if (== _leveltoload "None")
          _
          (elif (not (`LevelStreaming.IsLevelLoaded` (`GameplayStatics.GetStreamingLevel` _leveltoload)))
            (`GameplayStatics.LoadStreamLevel` _leveltoload true)
            (`KismetSystemLibrary.PrintString` (`KismetStringLibrary.Concat_StrStr` (`KismetStringLibrary.Conv_NameToString` _leveltoload) "Loaded"))))))))

(fn `UserConstructionScript`)