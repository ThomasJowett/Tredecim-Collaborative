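; BP_Rock is a configurable rock prop that sets its mesh and material look in the construction script.
; It creates a dynamic instance of RockMat, feeds its colour blend and tiling from Blueprint variables, and applies it to the Rock component.
; A RockType enum then selects one of five thin or fat static mesh variants.
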(fn `UserConstructionScript`
  (bind _rock (`self.Rock`))
  (bind _returnvalue (`PrimitiveComponent.CreateDynamicMaterialInstance` (`self.Rock`) 0 (`self.Rock_Mat`) "None"))
  (`MaterialInstanceDynamic.SetScalarParameterValue` _returnvalue "Colourblend" (`self.ColourParam`))
  (`MaterialInstanceDynamic.SetScalarParameterValue` _returnvalue "Tiling" (`self.TilingParam`))
  (`PrimitiveComponent.SetMaterial` (`self.Rock`) 0 _returnvalue)
  (switch `/Game/RockType` (`self.RockType`)
    (:`NewEnumerator0`
      (`StaticMeshComponent.SetStaticMesh` _rock "/Game/StaticMeshes/SM/SM_Rock_01.SM_Rock_01"))
    (:`NewEnumerator1`
      (`StaticMeshComponent.SetStaticMesh` _rock "/Game/StaticMeshes/SM/SM_Rock_05.SM_Rock_05"))
    (:`NewEnumerator2`
      (`StaticMeshComponent.SetStaticMesh` _rock "/Game/StaticMeshes/SM/SM_Rock_02.SM_Rock_02"))
    (:`NewEnumerator3`
      (`StaticMeshComponent.SetStaticMesh` _rock "/Game/StaticMeshes/SM/SM_Rock_03.SM_Rock_03"))
    (:`NewEnumerator4`
      (`StaticMeshComponent.SetStaticMesh` _rock "/Game/StaticMeshes/SM/SM_Rock_04.SM_Rock_04"))))